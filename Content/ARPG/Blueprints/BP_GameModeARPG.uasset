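; BP_GameModeARPG is the ARPG game mode that tracks which kinds of items the player has picked up.
; PickupItem adds the given item type to a set, so duplicates count once.
; HasAllItems reports completion by comparing the set's size to an enum's entry count.
; BeginPlay and Tick are empty, and leftover logic for possessing a pawn with player controller index 1 never runs.
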(event `self.ReceiveBeginPlay`)

(fn `Has All Items`
  (returns (Result :type Boolean))
  (return (== (`BlueprintSetLibrary.Set_Length` (`self.MyPickupSet`)) (enumcount `/Game/ARPG/Actor/E_PickType`))))

(fn `Pickup Item`
  (params (NewParam :type "/Game/ARPG/Actor/E_PickType Enum" :default "NewEnumerator0"))
  (`BlueprintSetLibrary.Set_Add` (`self.MyPickupSet`) NewParam))

(fn `UserConstructionScript`)