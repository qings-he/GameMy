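; Player controller for an ARPG that drives the Shinbi character, camera, pause and quest menus, and inventory.
; Movement supports camera-relative WASD or click-to-move via navmesh with a goal decal, plus stamina-like attribute-cost sprint and spring-arm orbit and zoom.
; BeginPlay loads items from a data table on authority and initializes inventory UI.
; UI events forward inventory, currency and NPC shop requests to the inventory manager or overlapped NPC.
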(event `Key|LeftShift`
  (params (Key :type "Key Structure"))
  (bind _shinbi (`self.Shinbi`))
  (bind _shinbi_2 (`self.Shinbi`))
  ;[1 1 1] 加速
  (:`Pressed`
    (if (>= (`.CurrenteValue_2_5120472D4ADFA7C850CAB88593C27016` (break `/Game/ARPG/Blueprints/Structure/S_Attribute` (`/Game/ARPG/Charactors/Shinbi/BP_CharaShinbi.GetAttribute` _shinbi "NewEnumerator2"))) 15.0)
      (set `CharacterMovementComponent.MaxWalkSpeed` 1600.0 (`Character.CharacterMovement` _shinbi_2))
      (`/Game/ARPG/Charactors/Shinbi/BP_CharaShinbi.ModifyAttribute` _shinbi_2 "NewEnumerator2" -15.0 0.0 false)))
  (:`Released`
    (set `CharacterMovementComponent.MaxWalkSpeed` 400.0 (`Character.CharacterMovement` _shinbi))))

(event `Key|MouseScrollUp`
  (params (Key :type "Key Structure"))
  (bind _springarm (`/Game/ARPG/Charactors/Shinbi/BP_CharaShinbi.SpringArm` (`self.Shinbi`)))
  ;[1 1 1] 镜头缩放
  (:`Pressed`
    (set `SpringArmComponent.TargetArmLength` (`KismetMathLibrary.FClamp` (- (`SpringArmComponent.TargetArmLength` _springarm) (`self.SpringArmLengthRate`)) 120.0 600.0) _springarm)))

(event `Key|MouseScrollDown`
  (params (Key :type "Key Structure"))
  (bind _springarm (`/Game/ARPG/Charactors/Shinbi/BP_CharaShinbi.SpringArm` (`self.Shinbi`)))
  ;[1 1 1] 镜头缩放
  (:`Pressed`
    (set `SpringArmComponent.TargetArmLength` (`KismetMathLibrary.FClamp` (+ (`SpringArmComponent.TargetArmLength` _springarm) (`self.SpringArmLengthRate`)) 150.0 600.0) _springarm)))

(event `InputAxis|MoveRight`
  (params (AxisValue :type "Float (single-precision)"))
  (bind _shinbi (`self.Shinbi`))
  (bind _bp_questmanager (`/Game/ARPG/Charactors/BP_CharactorARPG.BP_QuestManager` _shinbi))
  (bind (_returnvalue_location _returnvalue_rotation) (`KismetMathLibrary.BreakTransform` (`SceneComponent.GetRelativeTransform` (`/Game/ARPG/Charactors/Shinbi/BP_CharaShinbi.SpringArm` (`self.Shinbi`)))))
  ;[1 1 1] WASD
  (if (!= AxisValue 0.0)
    (if (`self.HasDecal`)
      (`self.StopMoveClearDecal`))
    (`Pawn.AddMovementInput` _shinbi (`KismetMathLibrary.GetRightVector` (`KismetMathLibrary.MakeRotator` 0.0 0.0 (.yaw _returnvalue_rotation))) AxisValue false)
    (if (`KismetSystemLibrary.IsValid` _bp_questmanager) :!label _label
      (`/Game/ARPG/Actor/Quest/QuestManagerComponent.OnPlayerMove` _bp_questmanager) ; 移动就更新
    )))

(event `InputAxis|MoveForward`
  (params (AxisValue :type "Float (single-precision)"))
  (bind _shinbi (`self.Shinbi`))
  (bind (_returnvalue_location _returnvalue_rotation) (`KismetMathLibrary.BreakTransform` (`SceneComponent.GetRelativeTransform` (`/Game/ARPG/Charactors/Shinbi/BP_CharaShinbi.SpringArm` _shinbi))))
  ;[1 1 1] WASD
  (if (!= AxisValue 0.0)
    ;;[1 1 1] 如果玩家改为手动输入就clear decal
    (if (`self.HasDecal`)
      (`self.StopMoveClearDecal`))
    (`Pawn.AddMovementInput` _shinbi (`KismetMathLibrary.GetForwardVector` (`KismetMathLibrary.MakeRotator` 0.0 0.0 (.yaw _returnvalue_rotation))) AxisValue false)
    (goto _label)))

(event `InputAxis|Turn`
  (params (AxisValue :type "Float (single-precision)"))
  (bind _springarm (`/Game/ARPG/Charactors/Shinbi/BP_CharaShinbi.SpringArm` (`self.Shinbi`)))
  (bind (_returnvalue_location _returnvalue_rotation) (`KismetMathLibrary.BreakTransform` (`SceneComponent.GetRelativeTransform` _springarm)))
  ;[1 1 1] 按住右键上下左右拖动屏幕
  (if (and (!= AxisValue 0.0) (`self.CanTurn`))
    (`SceneComponent.K2_SetRelativeRotation` _springarm (`KismetMathLibrary.MakeRotator` (.roll _returnvalue_rotation) (.pitch _returnvalue_rotation) (+ (.yaw _returnvalue_rotation) (* AxisValue 2.2))) false false)))

(event `Key|RightMouseButton`
  (params (Key :type "Key Structure"))
  ;[1 1 1] 按住右键上下左右拖动屏幕
  (:`Pressed`
    (set `self.CanTurn` true))
  (:`Released`
    (set `self.CanTurn` false)))

(event `InputAxis|Lookup`
  (params (AxisValue :type "Float (single-precision)"))
  (bind _springarm (`/Game/ARPG/Charactors/Shinbi/BP_CharaShinbi.SpringArm` (`self.Shinbi`)))
  (bind (_returnvalue_location _returnvalue_rotation) (`KismetMathLibrary.BreakTransform` (`SceneComponent.GetRelativeTransform` _springarm)))
  ;[1 1 1] 按住右键上下左右拖动屏幕
  (if (and (!= AxisValue 0.0) (`self.CanTurn`))
    (`SceneComponent.K2_SetRelativeRotation` _springarm (`KismetMathLibrary.MakeRotator` (.roll _returnvalue_rotation) (`KismetMathLibrary.FClamp` (+ (.pitch _returnvalue_rotation) (* AxisValue 2.2)) -145.0 45.0) (.yaw _returnvalue_rotation)) false false)))

(event `Key|LeftMouseButton`
  (params (Key :type "Key Structure"))
  (bind (_bblockinghit _binitialoverlap _time _distance _location _impactpoint _normal) (`GameplayStatics.BreakHitResult` (`self.GetHitResultUnderCursorByChannel` "TraceTypeQuery1")))
  ;[1 1 1] 鼠标点击，角色跟随移动
  (:`Pressed`
    (`self.StopMoveClearDecal`) ; 生成decal之前线检测是不是已经有一个了
    (bind _returnvalue (`|SpawnActorFromClass` "/Game/ARPG/Actor/BP_GoalDecal.BP_GoalDecal_C" (`KismetMathLibrary.MakeTransform` _location (`KismetMathLibrary.MakeRotFromZ` _normal)) "Undefined" "OverrideRootScale" null null))
    (set `self.CurrentGoaldecal` _returnvalue)
    (set `self.HasDecal` true)
    (`AIBlueprintHelperLibrary.SimpleMoveToLocation` self _location) ; 需要navigation mesh
    (`/Game/ARPG/Actor/Quest/QuestManagerComponent.OnPlayerMove` (`/Game/ARPG/Charactors/BP_CharactorARPG.BP_QuestManager` (`self.Shinbi`))) ; 移动就更新
  ))

(event `Key|P`
  (params (Key :type "Key Structure"))
  (bind _pausewidget (`self.PauseWidget`))
  (bind _appear (`/Game/ARPG/UI/WidgetBP/WB_PauseGameMenu.Appear` _pausewidget))
  (:`Pressed`
    (`/Engine/EditorBlueprintResources/StandardMacros.IsValid` _pausewidget
      (:`Is Valid`
        (if (not (`UserWidget.IsAnimationPlaying` _pausewidget _appear))
          (`Widget.SetVisibility` (`self.PauseWidget`) "Visible")
          (`UserWidget.PlayAnimation` _pausewidget _appear 0.0 1 "Forward" 1.0 false)
          (`KismetSystemLibrary.Delay` 0.75)
          (`GameplayStatics.SetGamePaused` true)
          (`WidgetBlueprintLibrary.SetInputMode_UIOnlyEx` self null))))))

(event `self.ReceiveBeginPlay`
  (bind _c_inventerymanager (`self.C_InventeryManager`))
  (`self.DisableInput` null)
  (bind _asbp_chara_shinbi (cast `/Game/ARPG/Charactors/Shinbi/BP_CharaShinbi` (`GameplayStatics.GetPlayerCharacter` 0)))
  (set `self.Shinbi` _asbp_chara_shinbi)
  (`WidgetBlueprintLibrary.SetInputMode_GameAndUIEx` self null "LockAlways")
  (`KismetSystemLibrary.Delay` 0.2)
  (`/Game/ARPG/Actor/Item/C_InventoryManager.Initialize Player CInventory` (`self.C_InventeryManager`) (`self.C_Inventery`))
  (`self.Server_LoadPlayerItem`)
  (`/Game/ARPG/Actor/Item/C_InventoryManager.InitializeUIMainPC` _c_inventerymanager (`/Game/ARPG/Charactors/Shinbi/BP_CharaShinbi.MainWidget` (`self.Shinbi`)))
  (`/Game/ARPG/Actor/Item/C_InventoryManager.Client_LoadInventory` _c_inventerymanager)
  (`self.EnableInput` null)
  (bind _returnvalue (`|CreateWidget` "/Game/ARPG/UI/WidgetBP/WB_PauseGameMenu.WB_PauseGameMenu_C" null self))
  (set `self.PauseWidget` _returnvalue)
  (`UserWidget.AddToViewport` _returnvalue 0)
  (`Widget.SetVisibility` _returnvalue "Collapsed"))

(event `Key|J`
  (params (Key :type "Key Structure"))
  (:`Pressed`
    (`/Game/ARPG/UI/WidgetBP/WB_Mission.PlayAnim` (`/Game/ARPG/UI/WidgetBP/WB_MainPC.WB_Mission` (`/Game/ARPG/Charactors/Shinbi/BP_CharaShinbi.MainWidget` (`self.Shinbi`))))
    (`GameplayStatics.SetGamePaused` true)))

(event `Key|B`
  (params (Key :type "Key Structure"))
  (bind _c_inventerymanager (`self.C_InventeryManager`))
  (:`Pressed`
    (if (`/Game/ARPG/Actor/Item/C_InventoryManager.IsInventoryOpen` _c_inventerymanager)
      (`/Game/ARPG/Actor/Item/C_InventoryManager.Client_CloseInventory` _c_inventerymanager)
      (else
        (`/Game/ARPG/Actor/Item/C_InventoryManager.Client_OpenInventory` _c_inventerymanager)))))

(event `/Game/ARPG/Actor/Item/BPI_HUD.UIClose Inventory Window`
  (bind _c_inventerymanager (`self.C_InventeryManager`))
  (`/Game/ARPG/Actor/Item/C_InventoryManager.Client_CloseInventory` _c_inventerymanager)
  (`/Game/ARPG/Actor/Item/C_InventoryManager.Server_CloseActorContainer` _c_inventerymanager))

(event `/Game/ARPG/Actor/Item/BPI_HUD.UIMoveInventoryItem`
  (params (FromItemIndex :type Integer) (ToItemIndex :type Integer))
  (`/Game/ARPG/Actor/Item/C_InventoryManager.Server_MoveInventoryItem` (`self.C_InventeryManager`) FromItemIndex ToItemIndex))

(event `/Game/ARPG/Actor/Item/BPI_HUD.UIOpen Food Store`
  (params (NPCActor :type "Actor Object Reference"))
  (`self.Server_OnActorUsed`))

(event `Server_OnActorUsed`
  (bind _c_inventerymanager (`self.C_InventeryManager`))
  (`self.On Actor Used`)
  (if (not (`/Game/ARPG/Actor/Item/C_InventoryManager.IsInventoryOpen` _c_inventerymanager))
    (`/Game/ARPG/Actor/Item/C_InventoryManager.Client_OpenInventory` _c_inventerymanager) ; 在打开商店时，如果玩家的背包没有打开就打开
  ))

(event `/Game/ARPG/Actor/Item/BPI_HUD.UIOpenTransactionWindow`
  (params (FromItemIndex :type Integer) (ToItemIndex :type Integer) (FromInventoryType :type "/Game/ARPG/Actor/Item/E_InventoryTy Enum" :default "NewEnumerator0") (ToInventoryType :type "/Game/ARPG/Actor/Item/E_InventoryTy Enum" :default "NewEnumerator0") (ItemInfo :type "/Game/ARPG/Actor/Item/S_InventoryItem Structure"))
  (`/Game/ARPG/Actor/Item/C_InventoryManager.CLient_OpenTransactionWindow` (`self.C_InventeryManager`) FromItemIndex ToItemIndex FromInventoryType ToInventoryType ItemInfo))

(event `/Game/ARPG/Actor/Item/BPI_HUD.AddMora`
  (params (Mora :type Integer))
  (`/Game/ARPG/Actor/Item/C_InventoryManager.Client_AddMora` (`self.C_InventeryManager`) Mora))

(event `/Game/ARPG/Actor/Item/BPI_HUD.UISplitInventoryItem`
  (params (FromInventoryType :type "/Game/ARPG/Actor/Item/E_InventoryTy Enum" :default "NewEnumerator0") (ToInventoryType :type "/Game/ARPG/Actor/Item/E_InventoryTy Enum" :default "NewEnumerator0") (FromItemIndex :type Integer) (ToItemIndex :type Integer) (Amount :type Integer))
  (`/Game/ARPG/Actor/Item/C_InventoryManager.Server_SplitInventoryItem` (`self.C_InventeryManager`) FromInventoryType ToInventoryType FromItemIndex ToItemIndex Amount))

(event `Key|Seven`
  (params (Key :type "Key Structure"))
  (:`Pressed`
    (`/Game/ARPG/Actor/Item/C_InventoryManager.Client_AddMora` (`self.C_InventeryManager`) -1000)))

(event `Key|Eight`
  (params (Key :type "Key Structure"))
  (:`Pressed`
    (`/Game/ARPG/Actor/Item/C_InventoryManager.Client_AddMora` (`self.C_InventeryManager`) 1000)))

(fn `GetPlayerState`
  (returns (Level :type Integer) (Mora :type Integer))
  (bind _c_inventerymanager (`self.C_InventeryManager`))
  (return (`/Game/ARPG/Actor/Item/C_InventoryManager.Level` _c_inventerymanager) (`/Game/ARPG/Actor/Item/C_InventoryManager.Mora` _c_inventerymanager)))

(fn `GetToolTip`
  (params (ID :type Name))
  (returns (ItemInfo :type "/Game/ARPG/Actor/Item/S_InventoryItem Structure"))
  (bind _returnvalue (`|GetDataTableRow` "/Game/ARPG/Actor/Item/DT_ItemList.DT_ItemList" ID)
    (:`then`
      (return _returnvalue))))

(fn `GetUsableActor`
  (returns (`Hit Other Actor` :type "Actor Object Reference"))
  (bind _hit_other_actor (`/Game/ARPG/Charactors/Shinbi/BP_CharaShinbi.Hit Other Actor` (`self.Shinbi`)))
  (`/Engine/EditorBlueprintResources/StandardMacros.IsValid` _hit_other_actor
    (:`Is Valid`
      (return _hit_other_actor))
    (:`Is Not Valid`
      (return null))))

(fn `On Actor Used`
  (`/Engine/EditorBlueprintResources/ActorMacros.Switch Has Authority`
    (:`Authority`
      (bind _hit_other_actor (`self.GetUsableActor`)) ; 得到Overlap到的可用NPC。打开商店时需要获得NPC信息
      (`/Engine/EditorBlueprintResources/StandardMacros.IsValid` _hit_other_actor
        (:`Is Valid`
          (message `/Game/ARPG/Actor/Item/BPI_UsableActorContainer.On Actor Used` _hit_other_actor self) ; NPC里面的接口实现时用NPC并打开了商店
        )))))

(fn `Server_LoadPlayerItem`
  (locals (LocalInventory :type "Array of /Game/ARPG/Actor/Item/S_InventoryItem Structure"))
  (`/Engine/EditorBlueprintResources/ActorMacros.Switch Has Authority` ; 交换机具有授权实例。用来判断是不是Server
    (:`Authority`
      (for _array_element (`self.InventoryID`)
        (bind (_id _amount) (break `/Game/ARPG/Actor/Item/S_InventoryID` _array_element))
        (bind _returnvalue (`|GetDataTableRow` "/Game/ARPG/Actor/Item/DT_ItemList.DT_ItemList" _id) ; 返回此表此行（一个结构体）
          (:`then`
            (bind _structout (setmembers `/Game/ARPG/Actor/Item/S_InventoryItem` :`StructRef` _returnvalue :`Amount` _amount)) ; 修改此结构体的成员变量
            (`KismetArrayLibrary.Array_Add` (`local.LocalInventory`) _structout) ; 从数据表读取出来，然后存入此函数内
          )))
      (`/Game/ARPG/Actor/Item/C_Inventory.Load Inventory Item` (`self.C_Inventery`) (`/Game/ARPG/Actor/Item/C_InventoryManager.InventorySlot` (`self.C_InventeryManager`)) (`local.LocalInventory`)) ; 装载到Client
    )))

(fn `StopMoveClearDecal`
  (bind _currentgoaldecal (`self.CurrentGoaldecal`))
  (`/Engine/EditorBlueprintResources/StandardMacros.IsValid` _currentgoaldecal
    (:`Is Valid`
      (`MovementComponent.StopMovementImmediately` (`Character.CharacterMovement` (`self.Shinbi`)))
      (`self.K2_DestroyActor` _currentgoaldecal)
      (set `self.HasDecal` false))))

(fn `UserConstructionScript`)