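; BP_Mora is a currency pickup actor that automatically flies to the player and credits its Mora amount.
; After a short random delay from spawn, it stops sphere physics and a timeline lerps it from its resting location toward the player's current position.
; On finish, it plays a coin sound, calls ClientAddMora on the BP_PlayerControllerARPG inventory manager and destroys itself.
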(event `self.ReceiveBeginPlay`
  (`KismetSystemLibrary.Delay` (`KismetMathLibrary.RandomFloatInRange` 0.5 1.2))
  (`PrimitiveComponent.SetSimulatePhysics` (`self.Sphere`) false)
  (set `self.InitialLocation` (`self.K2_GetActorLocation`))
  (bind (_direction _newtrack_0) (`Timeline|MoveToPlayer`)
    (:`Update`
      (`self.K2_SetActorLocation` (`KismetMathLibrary.VLerp` (`self.InitialLocation`) (`self.K2_GetActorLocation` (`self.Player`)) _newtrack_0)))
    (:`Finished`
      (`self.FInishCollect`))))

(event `FInishCollect`
  (bind _player (`self.Player`))
  (`GameplayStatics.PlaySoundAtLocation` "/Game/ARPG/Audio/Coins_10_Cue.Coins_10_Cue" (`self.K2_GetActorLocation` _player) (struct) 1.0 1.0 0.0 null null null)
  (`/Game/ARPG/Actor/Item/C_InventoryManager.Client_AddMora` (`/Game/ARPG/Blueprints/BP_PlayerControllerARPG.C_InventeryManager` (cast `/Game/ARPG/Blueprints/BP_PlayerControllerARPG` (`Pawn.GetController` _player) :!pure true)) (`self.Mora`))
  (`self.K2_DestroyActor`))

(fn `UserConstructionScript`)