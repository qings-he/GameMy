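; BP_Pickup is a collectible flower for the ARPG, with red, green and blue variants set by the PickTy value.
; The Construction Script picks the matching flower mesh, and Tick bobs it vertically with a time-based sine wave.
; When BP_CharaShinbi overlaps it, it passes its type to BP_GameModeARPG's PickupItem, then destroys itself.
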(event `self.ReceiveActorBeginOverlap`
  (params (OtherActor :type "Actor Object Reference"))
  (cast `/Game/ARPG/Charactors/Shinbi/BP_CharaShinbi` OtherActor)
  (`|ExecutionSequence`
    (:`then_0`
      (bind _asbp_game_mode_arpg (cast `/Game/ARPG/Blueprints/BP_GameModeARPG` (`GameplayStatics.GetGameMode`)))
      (`/Game/ARPG/Blueprints/BP_GameModeARPG.Pickup Item` _asbp_game_mode_arpg (`self.PickTy`)))
    (:`then_1`
      (`self.K2_DestroyActor`) ; Target默认是BP_Pickup自己
    )))

(event `self.ReceiveTick`
  (params (DeltaSeconds :type "Float (single-precision)"))
  (`SceneComponent.K2_SetRelativeLocation` (`self.FlowerCup1`) (`KismetMathLibrary.MakeVector` 0.0 0.0 (* (`KismetMathLibrary.Sin` (* (`GameplayStatics.GetTimeSeconds`) 2.0)) 20.0)) false false))

(fn `UserConstructionScript`
  (bind _flowercup1 (`self.FlowerCup1`))
  (switch `/Game/ARPG/Actor/E_PickType` (`self.PickTy`)
    (:`NewEnumerator0`
      (`StaticMeshComponent.SetStaticMesh` _flowercup1 "/Game/ARPG/StaticMesh/FlowerCup1.FlowerCup1"))
    (:`NewEnumerator1`
      (`StaticMeshComponent.SetStaticMesh` _flowercup1 "/Game/ARPG/StaticMesh/FlowerCup2_3.FlowerCup2_3"))
    (:`NewEnumerator2`
      (`StaticMeshComponent.SetStaticMesh` _flowercup1 "/Game/ARPG/StaticMesh/FlowerCup3_2.FlowerCup3_2"))))