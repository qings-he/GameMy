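; BP_TargetObject is a base actor for interactable objects that display a name and interaction prompt through a widget component.
; On BeginPlay it writes its Name and Interact text into the WB_Interaction widget and colors the name green.
; Overlap begin and end events show and hide the widget, while OnInteractwith is left empty for child classes to implement.
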(event `/Game/ARPG/Blueprints/Interface/BPI_Interaction.OnInteractWith`
  (params (Character :type "/Game/ARPG/Charactors/Shinbi/BP_CharaShinbi Object Reference")))

(event `self.ReceiveBeginPlay`
  (bind _aswb_interaction (cast `/Game/ARPG/UI/WidgetBP/WB_Interaction` (`WidgetComponent.GetUserWidgetObject` (`self.Widget`)) :!pure true))
  (bind _name (`/Game/ARPG/UI/WidgetBP/WB_Interaction.Name` _aswb_interaction))
  (`TextBlock.SetText` _name (`self.Name`))
  (`TextBlock.SetColorAndOpacity` _name (make `SlateColor` (struct :`G` 1.0 :`B` 0.016807 :`A` 1.0)))
  (`TextBlock.SetText` (`/Game/ARPG/UI/WidgetBP/WB_Interaction.Interact` _aswb_interaction) (`self.Interact`)))

(event `/Game/ARPG/Blueprints/Interface/BPI_Interaction.BeginOverlapTargetObject`
  (`SceneComponent.SetVisibility` (`self.Widget`) true false))

(event `/Game/ARPG/Blueprints/Interface/BPI_Interaction.EndOverlapTargetObject`
  (`SceneComponent.SetVisibility` (`self.Widget`) false false))

(fn `UserConstructionScript`)