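; Base weapon actor for the ARPG that applies its wielder's damage stats through overlap hits.
; On BeginPlay its capsule collision is disabled, and nothing in this graph re-enables it.
; On overlap, only player character 0 passes the check, despite a comment describing a non-wielder test.
; If that actor implements BPI_Damage, it receives the WeaponInstigator's physical, magic and critical attributes via ReceiveDamageMessage.
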(event `self.ReceiveBeginPlay`
  (bind _capsule (`self.Capsule`))
  (`PrimitiveComponent.IgnoreActorWhenMoving` _capsule null true)
  (`PrimitiveComponent.SetCollisionEnabled` _capsule "NoCollision"))

(event `self.ReceiveActorBeginOverlap`
  (params (OtherActor :type "Actor Object Reference"))
  (bind (_currenthealth _maxhealth _physicaldamage _criticalchance _magicdamage _physicaldefence _magicdefence _criticaldamage) (break `/Game/ARPG/Charactors/Enemies/S_EnemyAttribute` (`/Game/ARPG/Charactors/Enemies/BP_BaseEnemy.Attribute` (`self.WeaponInstigator`))))
  (if (and (== OtherActor (`GameplayStatics.GetPlayerCharacter` 0)) (`KismetSystemLibrary.DoesImplementInterface` OtherActor "/Game/ARPG/Blueprints/Interface/BPI_Damage.BPI_Damage_C"))
    (message `/Game/ARPG/Blueprints/Interface/BPI_Damage.ReceiveDamage` OtherActor _criticalchance _physicaldamage _criticaldamage _magicdamage)))

(fn `UserConstructionScript`)