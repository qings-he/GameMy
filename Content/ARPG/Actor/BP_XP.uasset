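; BP_XP is an experience pickup actor that flies to the player and grants XP.
; After a short random delay on spawn it turns off physics on its sphere and records its location.
; A timeline then lerps it from that spot to the player's current position, so it tracks a moving target.
; When the timeline finishes, it destroys itself and adds its XP value, assigned at spawn, to the player.
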(event `self.ReceiveBeginPlay`
  (`KismetSystemLibrary.Delay` (`KismetMathLibrary.RandomFloatInRange` 0.5 1.2))
  (`PrimitiveComponent.SetSimulatePhysics` (`self.Sphere`) false)
  (set `self.InitialLocation` (`self.K2_GetActorLocation`))
  (bind (_direction _newtrack_0) (`Timeline|MoveToPlayer`)
    (:`Update`
      (`self.K2_SetActorLocation` (`KismetMathLibrary.VLerp` (`self.InitialLocation`) (`self.K2_GetActorLocation` (`self.Player`)) _newtrack_0)))
    (:`Finished`
      (`self.FInishCollect`))))

(event `FInishCollect`
  (`self.K2_DestroyActor`)
  (`/Game/ARPG/Charactors/Shinbi/BP_CharaShinbi.AddXP` (`self.Player`) (`self.XP`)))

(fn `UserConstructionScript`)