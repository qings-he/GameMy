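; BP_Door is a double door that opens only when the ARPG game mode reports all items collected.
; On BeginPlay it spawns ten random-type BP_Pickup actors at random positions within fixed bounds.
; Overlapping the Were component plays a timeline that rotates both leaves and tints their dynamic materials, and leaving reverses it.
; A cross product against the player's position sets the sign of the timeline alpha, choosing the swing direction.
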(event `self.ReceiveBeginPlay`
  (for _ (range 1 11)
    (`|SpawnActorFromClass` "/Game/ARPG/Actor/BP_Pickup.BP_Pickup_C" (`KismetMathLibrary.MakeTransform` (`KismetMathLibrary.MakeVector` (`KismetMathLibrary.RandomFloatInRange` -1287.0 -1725.0) (`KismetMathLibrary.RandomFloatInRange` 3000.0 3900.0) (`KismetMathLibrary.RandomFloatInRange` -528.0 -600.0))) "Undefined" "OverrideRootScale" null (cast `/Game/ARPG/Actor/E_PickType` (`KismetMathLibrary.Conv_IntToByte` (`KismetMathLibrary.RandomIntegerInRange` 0 (- (enumcount `/Game/ARPG/Actor/E_PickType`) 1)))) null)))

(event `self.were.OnComponentBeginOverlap`
  (params (OverlappedComponent :type "PrimitiveComponent Object Reference") (OtherActor :type "Actor Object Reference") (OtherComp :type "PrimitiveComponent Object Reference") (OtherBodyIndex :type Integer) (bFromSweep :type Boolean) (SweepResult :type "HitResult Structure (by ref)"))
  (bind _asbp_game_mode_arpg (cast `/Game/ARPG/Blueprints/BP_GameModeARPG` (`GameplayStatics.GetGameMode`)))
  (bind _result (`/Game/ARPG/Blueprints/BP_GameModeARPG.Has All Items` _asbp_game_mode_arpg))
  (if _result
    (`self.DoorPN`)
    (bind (_direction _newtrack_0) (`Timeline|Timeline_0` :!label _label)
      (:`Update`
        (`|ExecutionSequence`
          (:`then_0`
            (bind _returnvalue (* _newtrack_0 (`self.bDoor`)))
            (`SceneComponent.K2_SetRelativeRotation` (`self.StaticMesh`) (`KismetMathLibrary.MakeRotator` 0.0 0.0 (`KismetMathLibrary.Lerp` 0.0 -90.0 _returnvalue)) false false)
            (`SceneComponent.K2_SetRelativeRotation` (`self.StaticMesh1`) (`KismetMathLibrary.MakeRotator` 0.0 0.0 (`KismetMathLibrary.Lerp` -180.0 -90.0 _returnvalue)) false false))
          (:`then_1`
            (bind _returnvalue_2 (`KismetMathLibrary.LinearColorLerp` (struct :`R` 0.215861 :`G` 0.215861 :`B` 0.215861) (struct :`R` 0.670833 :`G` 0.255586 :`B` 0.336215 :`A` 1.0) _returnvalue))
            (`MaterialInstanceDynamic.SetVectorParameterValue` (`self.MI_Door`) "Param" _returnvalue_2)
            (`MaterialInstanceDynamic.SetVectorParameterValue` (`self.MI_Door1`) "Param" _returnvalue_2)))))))

(event `self.were.OnComponentEndOverlap`
  (params (OverlappedComponent :type "PrimitiveComponent Object Reference") (OtherActor :type "Actor Object Reference") (OtherComp :type "PrimitiveComponent Object Reference") (OtherBodyIndex :type Integer))
  (goto _label :!via `Reverse`))

(event `DoorPN`
  (bind _staticmesh (`self.StaticMesh`))
  (if (>= (.z (`KismetMathLibrary.Cross_VectorVector` (- (`SceneComponent.K2_GetComponentLocation` _staticmesh) (`self.K2_GetActorLocation` (`GameplayStatics.GetPlayerCharacter` 0))) (`SceneComponent.GetForwardVector` _staticmesh))) 0.0)
    (set `self.bDoor` 1.0)
    (else
      (set `self.bDoor` -1.0))))

(fn `UserConstructionScript`
  (bind _returnvalue (`PrimitiveComponent.CreateDynamicMaterialInstance` (`self.StaticMesh`) 0 null "None")) ; Source Material默认是mesh自带的拿个
  (set `self.MI_Door` _returnvalue)
  (bind _returnvalue_2 (`PrimitiveComponent.CreateDynamicMaterialInstance` (`self.StaticMesh1`) 0 null "None")) ; Source Material默认是mesh自带的拿个
  (set `self.MI_Door1` _returnvalue_2))