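; BP_BaseQuest is the base quest for the ARPG, tracking one quest's active and completed subgoals by index into QuestInfo.
; It seeds starting subgoals and can step to the next index.
; CompleteSubGoal records results and updates quest and mission widgets.
; Once none remain active, it loads a completed subgoal's following branch, polling with a short Delay before rebuilding widgets, or plays the quest's hide animation.
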(event `UpdateCompletedSubgoal`
  (bind _manager_wbquest (`self.Manager_WBQuest`))
  (bind _manager_wbquest_2 (`self.Manager_WBQuest`))
  (bind _output (`|GetArrayItem` (`/Game/ARPG/Actor/Quest/WB_Quest.SubGoalWidgets` _manager_wbquest)))
  (for _array_element (`self.CompletedSubGoalInfo`)
    (bind ((`SubgoalInfo_8_7D4CA68C4DC5160394F643B4B89CC14B` _subgoalinfo)) (break `/Game/ARPG/Actor/Quest/S_CompletedSubgoalInfo` _array_element))
    (bind ((`FollowingSubGoalIndices_44_70F6B50644FFE2DAFAC0D3A3486FC478` _followingsubgoalindices) (`HasFollowingIndex_46_AB667F874122A02D542EF096372CAE2D` _hasfollowingindex)) (break `/Game/ARPG/Actor/Quest/S_SubGoalInfo` _subgoalinfo))
    (if _hasfollowingindex
      (set `self.HasFollowing` _hasfollowingindex) ; 先暂存
      (setmembers `/Game/ARPG/Actor/Quest/S_SubGoalInfo` :`StructRef` _subgoalinfo :`HasFollowingIndex` false) ; 已经完成的小分支后有Following，再置空
      (`KismetArrayLibrary.Array_Clear` (`self.CurrentSubGoalInfo`)) ; 先清空
      (`KismetArrayLibrary.Array_Clear` (`self.CurrentSubGoalIndices`))
      (for (_array_element_2 _array_index) _followingsubgoalindices
        (`KismetArrayLibrary.Array_Add` (`self.CurrentSubGoalIndices`) _array_index) ; 再把Following添加进去
        (`KismetArrayLibrary.Array_Add` (`self.CurrentHuntedAmounts`))
        (`KismetArrayLibrary.Array_Add` (`self.CurrentSubGoalInfo`) (`|GetArrayItem` (`.SubGoalInfo_17_5A3C121F4194D20DB591DD953A37967E` (break `/Game/ARPG/Actor/Quest/S_QuestInfo` (`self.QuestInfo`))) _array_element_2)) ; 添加到当前小分支数组
      )
      (break)))
  (if (`self.HasFollowing`)
    (`/Game/ARPG/Actor/Quest/WB_Quest.PlaySubgoal` _manager_wbquest false) ; 完成任务后（所有小分支）后播放隐藏动画，然后再更新为Following
    (if (`KismetSystemLibrary.IsValid` _output) :!label _label
      (`KismetSystemLibrary.Delay` 0.01)
      (goto _label)
      (else
        (`/Game/ARPG/Actor/Quest/WB_Quest.Generate Sub Goal` _manager_wbquest_2)
        (`/Game/ARPG/Actor/Quest/WB_Quest.Select Sub Goal` _manager_wbquest_2 _output) ; 重新生成小分支后要更新选择的小分支（更新当前小分支）
        (`/Game/ARPG/Actor/Quest/WB_Quest.PlaySubgoal` _manager_wbquest_2 true)))
    (else
      (`/Game/ARPG/Actor/Quest/WB_Quest.PlayQuest` _manager_wbquest false) ; 任务已经完成（没有小分支，也没有Following）
    )))

(fn `Complete Sub Goal`
  (params (SubgoalIndex :type Integer) (Success :type Boolean))
  (locals (LCompleteSubgoalIndex :type Integer) (LCompletedSubGoalInfo :type "/Game/ARPG/Actor/Quest/S_SubGoalInfo Structure") (LocalSuccess :type Boolean))
  (bind _returnvalue (`KismetArrayLibrary.Array_Find` (`self.CurrentSubGoalIndices`) (`local.LCompleteSubgoalIndex`)))
  (set `local.LocalSuccess` Success)
  (set `local.LCompleteSubgoalIndex` SubgoalIndex)
  (if (`KismetArrayLibrary.Array_Contains` (`self.CurrentSubGoalIndices`) (`local.LCompleteSubgoalIndex`))
    (`/Game/ARPG/Actor/Quest/WB_Subgoal.Disable Botton` (`|GetArrayItem` (`/Game/ARPG/Actor/Quest/WB_Quest.SubGoalWidgets` (`self.Manager_WBQuest`)) _returnvalue) (`local.LocalSuccess`)) ; 已经完成的小分支的下标存在，则禁用此小分支的选择按钮
    (`KismetArrayLibrary.Array_RemoveItem` (`self.CurrentHuntedAmounts`) _returnvalue) ; 删除已经完成的小分支（若此小分支是Hunt类型的）
    (`KismetArrayLibrary.Array_RemoveItem` (`self.CurrentSubGoalIndices`) (`local.LCompleteSubgoalIndex`)) ; 删除已经完成的小分支在Current数组里的下标
    (bind _output_get (set `local.LCompletedSubGoalInfo` (`|GetArrayItem` (`.SubGoalInfo_17_5A3C121F4194D20DB591DD953A37967E` (break `/Game/ARPG/Actor/Quest/S_QuestInfo` (`self.QuestInfo`))) (`local.LCompleteSubgoalIndex`)))) ; 已经完成的小分支
    (`KismetArrayLibrary.Array_Add` (`self.CompletedSubGoalInfo`) (make `/Game/ARPG/Actor/Quest/S_CompletedSubgoalInfo` (`local.LocalSuccess`) (`local.LCompleteSubgoalIndex`) _output_get)) ; 导入对应的集合（输出为小分支的下标）
    (`KismetArrayLibrary.Array_RemoveItem` (`self.CurrentSubGoalInfo`) (`local.LCompletedSubGoalInfo`)) ; 删除已经完成的小分支的info
    (if (not (`KismetArrayLibrary.Array_IsValidIndex` (`self.CurrentSubGoalIndices`)))
      (`self.UpdateCompletedSubgoal`) ; 没有小分支了，任务完成（删除所有小分支，添加Following）
      (else
        (if (`self.Selected In Mission`)
          (`/Game/ARPG/UI/WidgetBP/WB_Mission.Generat Subgoal` (`/Game/ARPG/UI/WidgetBP/WB_MainPC.WB_Mission` (`self.Manager_MainPC`))))
        (if (and (== (`self.SelectedSubGoalIndex`) (`local.LCompleteSubgoalIndex`)) (== (`/Game/ARPG/Actor/Quest/QuestManagerComponent.CurrentQuest` (`self.QuestManager`)) self))
          (`/Game/ARPG/Actor/Quest/WB_Quest.Select Sub Goal` (`self.Manager_WBQuest`) (`|GetArrayItem` (`/Game/ARPG/Actor/Quest/WB_Quest.SubGoalWidgets` (`self.Manager_WBQuest`)) (`|GetArrayItem` (`self.CurrentSubGoalIndices`)))))))))

(fn `Goto Next Subgoal`
  (returns (Success :type Boolean))
  (locals (LocalNextIndex :type Integer :default 0))
  (bind _currentsubgoalindices (`self.CurrentSubGoalIndices`))
  (bind _returnvalue (+ (`.MaxValue` (`KismetMathLibrary.MaxOfIntArray` (`self.CurrentSubGoalIndices`))) 1))
  (if (<= _returnvalue (`KismetArrayLibrary.Array_LastIndex` (`.SubGoalInfo_17_5A3C121F4194D20DB591DD953A37967E` (break `/Game/ARPG/Actor/Quest/S_QuestInfo` (`self.QuestInfo`)))))
    (set `local.LocalNextIndex` _returnvalue) ; 没有超过，下面还有小分支，那就先把它的下标存下来
    (`KismetArrayLibrary.Array_Clear` _currentsubgoalindices)
    (`KismetArrayLibrary.Array_Add` _currentsubgoalindices (`local.LocalNextIndex`))
    (`self.Update Sub Goals Info`) ; 任务信息改变后要手动刷新
    (return true)
    (else
      (return false) ; 大于了最后一个小分支的下标，那就做完了所有小分支，不用前往下一个分支了，所以前往失败
    )))

(fn `Selected In Mission`
  (returns (QuestEqual :type Boolean))
  (bind _selectquest (`/Game/ARPG/UI/WidgetBP/WB_Mission.SelectQuest` (`/Game/ARPG/UI/WidgetBP/WB_MainPC.WB_Mission` (`self.Manager_MainPC`))))
  (return (and (`KismetSystemLibrary.IsValid` _selectquest) (== _selectquest (`/Game/ARPG/Actor/Quest/QuestManagerComponent.CurrentQuest` (`self.QuestManager`))))))

(fn `Setup Starting Sub Goals`
  (bind _startsubgoalindices (`self.StartSubGoalIndices`))
  (`KismetArrayLibrary.Array_Clear` (`self.CurrentSubGoalIndices`)) ; 先清除当前子任务下标集合
  (set `self.CurrentSubGoalIndices` _startsubgoalindices)
  (`KismetArrayLibrary.Array_Resize` (`self.CurrentHuntedAmounts`) (`KismetArrayLibrary.Array_Length` _startsubgoalindices)) ; 将数组大小调整为指定大小
  (set `self.CurrentDescription` (`.Description_4_3BF6BA9D41566759E18A398D001A8706` (break `/Game/ARPG/Actor/Quest/S_QuestInfo` (`self.QuestInfo`))))
  (`self.Update Sub Goals Info`)
  (return))

(fn `Update Sub Goals Info`
  (`KismetArrayLibrary.Array_Clear` (`self.CurrentSubGoalInfo`)) ; 先清空当前的所有子任务（任务小分支）
  (for _array_element (`self.CurrentSubGoalIndices`)
    (`KismetArrayLibrary.Array_Add` (`self.CurrentSubGoalInfo`) (`|GetArrayItem` (`.SubGoalInfo_17_5A3C121F4194D20DB591DD953A37967E` (break `/Game/ARPG/Actor/Quest/S_QuestInfo` (`self.QuestInfo`))) _array_element)) ; 添加到当前任务的小分支任务集合里，完成小分支的更新
  )
  (return))

(fn `UserConstructionScript`)