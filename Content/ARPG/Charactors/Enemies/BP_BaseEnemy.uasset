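; Base ARPG enemy character with level-scaled attributes, an attached weapon and a health/level widget shown near the player, colored by level difference.
; Pawn sensing and incoming hits set the Blackboard target and switch BehaviorComponent states.
; Damage applies defense and criticals, showing damage text, hit reactions and critical knockback.
; Death notifies the player's quest manager, waits out the montage, drops XP and Mora, triggers the respawn actor and destroys itself.
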(event `self.ReceiveBeginPlay`
  (bind _returnvalue (`AIBlueprintHelperLibrary.GetBlackboard` null))
  (bind _papersprite (`self.PaperSprite`))
  (`parent.ReceiveBeginPlay`)
  (`self.UpdateAttribute`)
  (`self.CreateWeapon`)
  (`self.SetOwner` (`GameplayStatics.GetPlayerCharacter` 0)) ; 设置此Actor的所有者，该Actor主要用于网络复制
  (`PrimitiveComponent.SetOwnerNoSee` _papersprite true)
  (`SceneComponent.SetVisibility` _papersprite true false)
  (`self.SetHealth`)
  (set `CharacterMovementComponent.MaxWalkSpeed` 200.0 (`self.CharacterMovement`))
  (`BlackboardComponent.SetValueAsVector` _returnvalue "Origin" (`self.K2_GetActorLocation`)) ; 赋值传递给黑板
  (`BlackboardComponent.SetValueAsFloat` _returnvalue "RandomRange" (`self.RandomRange`))
  (`/Game/ARPG/Component/BehaviorComponent.SetBehavior` (`self.BehaviorComponent`) "NewEnumerator4")
  (bind _asbp_chara_shinbi (cast `/Game/ARPG/Charactors/Shinbi/BP_CharaShinbi` (`GameplayStatics.GetPlayerCharacter` 0) :!label _label)
    (:`then`
      (`self.Set Name and Level` (`/Game/ARPG/Charactors/Shinbi/BP_CharaShinbi.Level` _asbp_chara_shinbi))
      (add `/Game/ARPG/Charactors/Shinbi/BP_CharaShinbi.UpgradeForQuest` _asbp_chara_shinbi (`|CreateDelegate` :!event `Set Name and Level`)) ; 收到玩家发送来的升级消息后，更新颜色
      (set `self.Shinbi` _asbp_chara_shinbi))
    (:`CastFailed`
      (`KismetSystemLibrary.Delay` 2.0)
      (goto _label))))

(event `UpdateLevelColor`
  (params (Level :type Integer))
  (`self.Set Name and Level` Level))

(event `Reset`
  ;[1 1 1] 发现玩家
  (set `CharacterMovementComponent.MaxWalkSpeed` 200.0 (`self.CharacterMovement`))
  (`/Game/ARPG/Component/BehaviorComponent.SetBehavior` (`self.BehaviorComponent`) "NewEnumerator4")
  (goto _label_2 :!via `Reset`))

(event `self.PawnSensing.OnSeePawn`
  (params (Pawn :type "Pawn Object Reference"))
  ;[1 1 1] 发现玩家
  (if (== Pawn (`GameplayStatics.GetPlayerPawn` 0))
    (`BlackboardComponent.SetValueAsObject` (`AIBlueprintHelperLibrary.GetBlackboard` null) "Target" Pawn) ; 看见的Pawn是玩家
    (set `CharacterMovementComponent.MaxWalkSpeed` 400.0 (`self.CharacterMovement`)) ; 发现玩家后激动不已，加速
    (`/Engine/EditorBlueprintResources/StandardMacros.DoOnce` false :!label _label_2
      (:`Completed`
        (`/Game/ARPG/Component/BehaviorComponent.SetBehavior` (`self.BehaviorComponent`) "NewEnumerator5")
        (`GameplayStatics.PlaySoundAtLocation` "/Game/ARPG/Audio/Enemy_Gruntling/A_Guardian_Roar02_Cue.A_Guardian_Roar02_Cue" (`self.K2_GetActorLocation`) (struct) 1.0 1.0 0.0 null null null)))))

(event `Attack`
  (params (BTTask :type "/Game/ARPG/AI/BTTask/BTT_Attack Object Reference"))
  (`self.K2_SetActorRotation` (`KismetMathLibrary.FindLookAtRotation` (`self.K2_GetActorLocation`) (`self.K2_GetActorLocation` (`GameplayStatics.GetPlayerCharacter` 0))))
  (bind _returnvalue (`self.PlayAnimMontage` (`self.AttackMontage`)))
  (`KismetSystemLibrary.Delay` _returnvalue)
  (`/Game/ARPG/AI/BTTask/BTT_Attack.FinalAttack` BTTask))

(event `CreateWeapon`
  (bind _weapon (`self.Weapon`))
  (if (`KismetSystemLibrary.IsValidClass` _weapon)
    (bind _returnvalue (`|SpawnActorFromClass` _weapon (`KismetMathLibrary.MakeTransform` (0.0 0.0 0.0)) "AlwaysSpawn" "OverrideRootScale" null self null))
    (bind _output_get (set `self.CurrentWeapon` _returnvalue))
    (`self.K2_AttachToComponent` _output_get (`self.Mesh`) "WeaponSocket" "KeepRelative" "KeepRelative" "KeepRelative" true)))

(event `/Game/ARPG/Blueprints/Interface/BPI_Damage.ReceiveDamage`
  (params (CriticalChance :type "Float (single-precision)") (PhysicalDamage :type "Float (single-precision)") (CriticalDamage :type "Float (single-precision)") (MagicDamage :type "Float (single-precision)") (Attacker :type "Actor Object Reference"))
  (bind ((`PhysicalDefence_14_1028F0F34CEC7FBF8F53E6B9724D20E0` _physicaldefence) (`MagicDefence_16_F8E076B7433B3A3AF9E6AF8D88705C2D` _magicdefence)) (break `/Game/ARPG/Charactors/Enemies/S_EnemyAttribute` (`self.Attribute`)))
  (if (`self.IsAlive`)
    (set `self.CurrentAttacker` Attacker)
    (bind (_critical _damage) (`self.CalculateDamage` PhysicalDamage MagicDamage CriticalChance CriticalDamage _physicaldefence _magicdefence))
    (`|ExecutionSequence`
      (:`then_0`
        (if (not (`BlackboardComponent.GetValueAsBool` (`AIBlueprintHelperLibrary.GetBlackboard` null) "IsRuningBack"))
          (`self.PlayAnimMontage` (select `bool` _critical :`false` (`self.ReactLightMontage`) :`true` (`self.ReactHeavyMontage`)) 1.0 (`KismetStringLibrary.Conv_StringToName` (`KismetStringLibrary.Conv_IntToString` (`KismetMathLibrary.RandomInteger` 2))))
          (if _critical
            (`self.LaunchCharacter` (* (`self.GetActorForwardVector` (`GameplayStatics.GetPlayerCharacter` 0)) 300.0)) ; 暴击时击退敌人
          )))
      (:`then_1`
        (`self.ModifyAttribute` _critical (* _damage -1.0))))))

(event `ModifyAttribute`
  (params (Critical :type Boolean) (Damage :type "Float (double-precision)"))
  (bind _attribute (`self.Attribute`))
  (bind _behaviorcomponent (`self.BehaviorComponent`))
  (bind ((`CurrentHealth_3_B0275C554314227EF2295896EFC75994` _currenthealth)) (break `/Game/ARPG/Charactors/Enemies/S_EnemyAttribute` _attribute))
  ;[1 1 1] 收到玩家攻击，改变状态和行为
  (bind _returnvalue (`AddComponent|NODE_AddWC_OnDamage-0` :`bManualAttachment` true :`RelativeTransform` (`self.GetTransform`)))
  (`/Game/ARPG/Component/WC_OnDamage.SetDamageText` _returnvalue Damage false "NewEnumerator0" Critical)
  (setmembers `/Game/ARPG/Charactors/Enemies/S_EnemyAttribute` :`StructRef` _attribute :`CurrentHealth` (+ Damage _currenthealth))
  (`self.SetHealth`)
  (if (<= _currenthealth 0.0)
    (`/Game/ARPG/Component/BehaviorComponent.SetBehavior` _behaviorcomponent "NewEnumerator6")
    (else
      (`BlackboardComponent.SetValueAsObject` (`AIBlueprintHelperLibrary.GetBlackboard` null) "Target" (`self.CurrentAttacker`)) ; 设置行为时要用到黑板，要把数据设置过去
      (`/Game/ARPG/Component/BehaviorComponent.SetBehavior` _behaviorcomponent "NewEnumerator5"))))

(event `self.CheckShowEnemyInfo.OnComponentBeginOverlap`
  (params (OverlappedComponent :type "PrimitiveComponent Object Reference") (OtherActor :type "Actor Object Reference") (OtherComp :type "PrimitiveComponent Object Reference") (OtherBodyIndex :type Integer) (bFromSweep :type Boolean) (SweepResult :type "HitResult Structure (by ref)"))
  ;[1 1 1] 13米开外不可见EnemyInfoWB
  (if (`PrimitiveComponent.IsOverlappingActor` (`self.CheckShowEnemyInfo`) (`GameplayStatics.GetPlayerCharacter` 0))
    (`SceneComponent.SetVisibility` (`self.WBEnemyInfo`) true false)))

(event `self.CheckShowEnemyInfo.OnComponentEndOverlap`
  (params (OverlappedComponent :type "PrimitiveComponent Object Reference") (OtherActor :type "Actor Object Reference") (OtherComp :type "PrimitiveComponent Object Reference") (OtherBodyIndex :type Integer))
  ;[1 1 1] 13米开外不可见EnemyInfoWB
  (if (`PrimitiveComponent.IsOverlappingActor` (`self.CheckShowEnemyInfo`) (`GameplayStatics.GetPlayerCharacter` 0))
    (`SceneComponent.SetVisibility` (`self.WBEnemyInfo`) false false)))

(event `OnDead`
  (bind _currentweapon (`self.CurrentWeapon`))
  (bind _respawnactor (`self.RespawnActor`))
  (`/Game/ARPG/Actor/Quest/QuestManagerComponent.OnEnemyKill` (`/Game/ARPG/Charactors/BP_CharactorARPG.BP_QuestManager` (`self.Shinbi`)) (`GameplayStatics.GetObjectClass` self))
  (`SceneComponent.SetVisibility` (`self.WBEnemyInfo`) false false)
  (`SceneComponent.SetVisibility` (`self.PaperSprite`) false false)
  (`self.DetachFromControllerPendingDestroy`) ; 调用此函数可以安全地将pawn从其控制器中分离出来，因为我们知道我们很快就会被摧毁
  (`self.PlayAnimMontage` (`self.DeadMontage`) 1.0 (`KismetStringLibrary.Conv_StringToName` (`KismetStringLibrary.Conv_IntToString` (`KismetMathLibrary.RandomInteger` 7))))
  (if (not (`self.IsPlayMontage`)) :!label _label_3
    (`self.Spawn XPAnd Mora` (`KismetMathLibrary.RandomIntegerInRange` 1 5)) ; 在动画结束后，随机生成几个获得物特效
    (`/Engine/EditorBlueprintResources/StandardMacros.IsValid` _respawnactor
      (:`Is Valid`
        (`/Game/ARPG/Actor/BP_SpawnEnemy.SpawnEnemy` _respawnactor (make `/Game/ARPG/Actor/S_RespawnEnemy` (`self.SpawnTime`) (`GameplayStatics.GetObjectClass` self))))
      (:`Is Not Valid`
        _))
    (`self.K2_DestroyActor`)
    (`/Engine/EditorBlueprintResources/StandardMacros.IsValid` _currentweapon
      (:`Is Valid`
        (`self.K2_DestroyActor` _currentweapon)))
    (else
      (`KismetSystemLibrary.Delay` 0.01) ; 直到死亡动画播放结束
      (goto _label_3))))

(fn `IsAlive`
  (returns (NewParam :type Boolean))
  (return (> (`.CurrentHealth_3_B0275C554314227EF2295896EFC75994` (break `/Game/ARPG/Charactors/Enemies/S_EnemyAttribute` (`self.Attribute`))) 0.0)))

(fn `IsPlayMontage`
  (returns (NewParam :type Boolean))
  (return (`KismetSystemLibrary.IsValid` (`self.GetCurrentMontage` self))))

(fn `Set Name and Level`
  (params (PlayerLevel :type Integer))
  (bind _level (`self.Level`))
  (bind _level_2 (`/Game/ARPG/Charactors/Enemies/WB_Enemy.Level` (cast `/Game/ARPG/Charactors/Enemies/WB_Enemy` (`WidgetComponent.GetUserWidgetObject` (`self.WBEnemyInfo`)) :!pure true)))
  (set `self.XP_Points` (* (`self.XP_Points`) 1.3))
  (`TextBlock.SetText` _level_2 (`|FormatText` "Lv.{Level} {Name}" (`self.Level`) (`self.Name`)))
  (`TextBlock.SetColorAndOpacity` _level_2 (make `SlateColor` (select `bool` (< (+ PlayerLevel 5) _level) :`false` (select `bool` (> PlayerLevel (+ _level 1)) :`false` (`KismetMathLibrary.LinearColorLerpUsingHSV` (struct :`R` 1.0 :`A` 1.0) (struct :`R` 1.0 :`G` 1.0 :`B` 1.0 :`A` 1.0) (/ (`KismetMathLibrary.Conv_IntToDouble` PlayerLevel) (`KismetMathLibrary.Conv_IntToDouble` _level))) :`true` (struct :`R` 1.0 :`G` 1.0 :`B` 1.0 :`A` 1.0)) :`true` (struct :`R` 1.0 :`A` 1.0))))
  (return))

(fn `SetHealth`
  (bind ((`CurrentHealth_3_B0275C554314227EF2295896EFC75994` _currenthealth) (`MaxHealth_5_824A6FA04CE152E2ECDD08931BC0562D` _maxhealth)) (break `/Game/ARPG/Charactors/Enemies/S_EnemyAttribute` (`self.Attribute`)))
  (`ProgressBar.SetPercent` (`/Game/ARPG/Charactors/Enemies/WB_Enemy.HealthBar` (cast `/Game/ARPG/Charactors/Enemies/WB_Enemy` (`WidgetComponent.GetUserWidgetObject` (`self.WBEnemyInfo`)) :!pure true)) (/ _currenthealth _maxhealth))
  (return))

(fn `Spawn XPAnd Mora`
  (params (LastIndex :type Integer))
  (bind _returnvalue (`KismetMathLibrary.Conv_VectorToTransform` (`KismetMathLibrary.RandomPointInBoundingBox` (`self.K2_GetActorLocation`) (44.0 44.0 44.0))))
  (for _ (range 1 (+ LastIndex 1))
    (`|SpawnActorFromClass` "/Game/ARPG/Actor/BP_XP.BP_XP_C" _returnvalue "Undefined" "OverrideRootScale" null (`self.Shinbi`) (`self.XP_Points`) null)
    (`|SpawnActorFromClass` "/Game/ARPG/Actor/BP_Mora.BP_Mora_C" _returnvalue "Undefined" "OverrideRootScale" null (`self.Shinbi`) (`self.Mora`) null)
    (return)))

(fn `UpdateAttribute`
  (bind _attribute (`self.Attribute`))
  (bind (_currenthealth _maxhealth _physicaldamage _criticalchance _magicdamage _physicaldefence) (break `/Game/ARPG/Charactors/Enemies/S_EnemyAttribute` _attribute))
  (bind _returnvalue (* _maxhealth 1.2))
  (bind _returnvalue_2 (* _physicaldamage 1.4))
  (bind _returnvalue_3 (* _physicaldefence 1.3))
  (for _ (range 1 (+ (`self.Level`) 1))
    (setmembers `/Game/ARPG/Charactors/Enemies/S_EnemyAttribute` :`StructRef` _attribute :`CurrentHealth` _returnvalue :`MaxHealth` _returnvalue :`PhysicalDamage` _returnvalue_2 :`CriticalChance` (* _criticalchance 1.1) :`MagicDamage` _returnvalue_2 :`PhysicalDefence` _returnvalue_3 :`MagicDefence` _returnvalue_3)
    (set `self.XP_Points` (* (`self.XP_Points`) 1.3))
    (set `self.DropMora` (+ (`self.DropMora`) 12))
    (return)))

(fn `UserConstructionScript`
  (`parent.UserConstructionScript`))