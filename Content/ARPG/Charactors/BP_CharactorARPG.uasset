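; ARPG character Blueprint whose only logic is CalculateDamage, returning rounded damage and a critical flag unless AbsoluteDefence skips it.
; Physical and magic damage each get random variance, wider for magic, minus matching defence, falling back to 1 if non-positive.
; Both sequenced branches join at a shared critical roll, multiplier and return, so positive physical damage returns before magic is computed.
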(fn `CalculateDamage`
  (params (PhysicalDamage :type "Float (double-precision)") (MagicDamage :type "Float (double-precision)") (CriticalChance :type "Float (double-precision)") (CriticalDamage :type "Float (double-precision)") (PhysicalDefence :type "Float (double-precision)") (MagicDefence :type "Float (double-precision)") (AbsoluteDefence :type Boolean))
  (returns (Critical :type Boolean) (Damage :type "Float (double-precision)"))
  (locals (LPhysicalDamage :type "Float (double-precision)") (LMagicDamage :type "Float (double-precision)") (LDamage :type "Float (double-precision)") (HasCriticalChance :type Boolean))
  (bind _returnvalue (- (* MagicDamage (`KismetMathLibrary.RandomFloatInRange` 0.78 1.39)) MagicDefence))
  (bind _returnvalue_2 (- (* PhysicalDamage (`KismetMathLibrary.RandomFloatInRange` 0.9 1.1)) PhysicalDefence))
  (if (not AbsoluteDefence)
    (`|ExecutionSequence`
      (:`then_0`
        (if (> PhysicalDamage 0.0)
          (bind _output_get (set `local.LPhysicalDamage` (select `bool` (> _returnvalue_2 0.0) :`false` 1.0 :`true` _returnvalue_2)))
          (set `local.LDamage` (+ _output_get (stale _output_get_4)) :!label _label)
          (bind _output_get_2 (set `local.HasCriticalChance` (< (`KismetMathLibrary.RandomFloatInRange` 1.0 100.0) CriticalChance)))
          (bind _output_get_3 (set `local.LDamage` (* (`local.LDamage`) (select `bool` (`local.HasCriticalChance`) :`false` 1.0 :`true` CriticalDamage))))
          (return _output_get_2 (`KismetMathLibrary.Conv_IntToDouble` (`KismetMathLibrary.Round` _output_get_3)))))
      (:`then_1`
        (if (> MagicDamage 0.0)
          (bind _output_get_4 (set `local.LMagicDamage` (select `bool` (> _returnvalue 0.0) :`false` 1.0 :`true` _returnvalue)))
          (goto _label))))))

(fn `UserConstructionScript`)