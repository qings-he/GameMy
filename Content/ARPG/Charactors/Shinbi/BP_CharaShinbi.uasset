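; Player character Shinbi for the ARPG, handling double jump, melee combos, damage, interaction, quests and leveling.
; Loads SaveGame state on BeginPlay, then builds the main HUD and binds attribute widgets.
; A map of Health, Mana and Stamina structs feeds ModifyAttribute, which updates bars and pauses or resumes per-attribute regen timers, slowed in combat.
; Combos chain montages through buffered input; line traces send damage through BPI_Damage.
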(event `Regeneration`
  (bind _keys (`BlueprintMapLibrary.Map_Keys` (`self.Attributes`)))
  (for _array_element _keys
    (bind _value (`self.GetAttribute` _array_element))
    (bind ((`RegenInterval_25_85F391B240D6E6B8ADDF62B5AA9742EC` _regeninterval) (`RegenFuncName_30_D21768E4447A39058C082D855A3CDBCD` _regenfuncname)) (break `/Game/ARPG/Blueprints/Structure/S_Attribute` _value))
    (bind _returnvalue (`KismetSystemLibrary.K2_SetTimer` null _regenfuncname _regeninterval true))
    (bind _structout (setmembers `/Game/ARPG/Blueprints/Structure/S_Attribute` :`StructRef` _value :`RegenTimeHandle` _returnvalue))
    (`self.SetAttribute` _array_element _structout)
    (`self.Regen on Off` _array_element)))

(event `Upgrade`
  (params (Level :type Integer))
  (bind _charactermovement (`self.CharacterMovement`))
  (`self.UpgradeForQuest` Level)
  (bind _output_get (set `self.Level` Level))
  (set `/Game/ARPG/UI/WidgetBP/WB_CharactorBorder.LevelText` (`KismetTextLibrary.Conv_IntToText` _output_get) (`/Game/ARPG/UI/WidgetBP/WB_MainPC.WB_CharactorBorder` (`self.MainWidget`)))
  (if (not (<= Level 0))
    (`|ExecutionSequence`
      (:`then_0`
        (set `CharacterMovementComponent.MaxWalkSpeed` 0.0 _charactermovement)
        (`self.PlayAnimMontage` "/Game/ARPG/Charactors/Shinbi/Animation/Montage/Upgrade_HappyClap_Montage.Upgrade_HappyClap_Montage" 1.5)
        (`KismetSystemLibrary.Delay` 2.0)
        (set `CharacterMovementComponent.MaxWalkSpeed` 600.0 _charactermovement))
      (:`then_1`
        (bind _keys (`BlueprintMapLibrary.Map_Keys` (`self.Attributes`)))
        (for _array_element _keys
          (switch `/Game/ARPG/Blueprints/Enumeration/E_Attribute` _array_element ; 升级只会修改上限值，不会改当前值，当前值也可以改
            (:`NewEnumerator0`
              (`self.ModifyAttribute` "NewEnumerator0" 100.0 100.0) ; 升级时连带加上100当前血量
            )
            (:`NewEnumerator1`
              (`self.ModifyAttribute` "NewEnumerator1" 50.0 50.0))
            (:`NewEnumerator2`
              (`self.ModifyAttribute` "NewEnumerator2" 10.0 10.0)))))
      (:`then_2`
        (set `self.PhysicalDefence` (* (`self.PhysicalDefence`) 1.2))
        (set `self.PhysicalDamage` (* (`self.PhysicalDamage`) 1.3))
        (set `self.MagicDamage` (* (`self.MagicDamage`) 1.4))
        (set `self.MagicDefence` (* (`self.MagicDefence`) 1.1))))))

(event `self.ReceiveBeginPlay`
  (bind _mainwidget (`self.MainWidget`))
  (bind _level (`self.Level`))
  (bind _wb_level (`/Game/ARPG/UI/WidgetBP/WB_MainPC.WB_Level` _mainwidget))
  (bind _returnvalue (`GameplayStatics.DoesSaveGameExist` "SaveARPG"))
  (if _returnvalue
    (bind _returnvalue_2 (`GameplayStatics.LoadGameFromSlot` "SaveARPG"))
    (bind _assave_game_arpg (cast `/Game/ARPG/Blueprints/SaveGame_ARPG` _returnvalue_2)
      (:`then`
        (set `self.Attributes` (`/Game/ARPG/Blueprints/SaveGame_ARPG.PlayerAttribute` _assave_game_arpg))
        (set `self.Level` (`/Game/ARPG/Blueprints/SaveGame_ARPG.PLayerLevel` _assave_game_arpg))
        (set `/Game/ARPG/Actor/Item/C_InventoryManager.Mora` (`/Game/ARPG/Blueprints/SaveGame_ARPG.PlayerMora` _assave_game_arpg) (`/Game/ARPG/Blueprints/BP_PlayerControllerARPG.C_InventeryManager` (cast `/Game/ARPG/Blueprints/BP_PlayerControllerARPG` (`GameplayStatics.GetPlayerController` 0) :!pure true)))
        (`self.K2_SetActorLocation` (`/Game/ARPG/Blueprints/SaveGame_ARPG.PLayerLocation` _assave_game_arpg)))
      (:`CastFailed`
        _)))
  (set `/Game/ARPG/Actor/Quest/QuestManagerComponent.Shinbi` self (`self.BP_QuestManager`))
  (bind _returnvalue_3 (`|CreateWidget` "/Game/ARPG/UI/WidgetBP/WB_MainPC.WB_MainPC_C" null self))
  (bind _output_get (set `self.MainWidget` _returnvalue_3))
  (`self.SetupAttributeBar`)
  (`self.Updata Attribute` "NewEnumerator0")
  (`self.Updata Attribute` "NewEnumerator1")
  (`self.Regeneration`)
  (`UserWidget.AddToViewport` _output_get 0)
  (add `/Game/ARPG/UI/WidgetBP/WB_Level.UpdateLevel` _wb_level (`|CreateDelegate` :!event `Upgrade`)) ; shibi注册了这个事件，负责实现他
  (`/Game/ARPG/UI/WidgetBP/WB_Level.InitialLevel` _wb_level _level)
  (set `/Game/ARPG/UI/WidgetBP/WB_CharactorBorder.LevelText` (`KismetTextLibrary.Conv_IntToText` _level) (`/Game/ARPG/UI/WidgetBP/WB_MainPC.WB_CharactorBorder` _mainwidget)))

(event `Key|O`
  (params (Key :type "Key Structure"))
  (bind _bp_questmanager (`self.BP_QuestManager`))
  (:`Pressed`
    (`/Game/ARPG/Actor/Quest/QuestManagerComponent.Add Quest` _bp_questmanager "/Game/ARPG/Actor/Quest/BP_TestQuest.BP_TestQuest_C" false)
    (`/Game/ARPG/Actor/Quest/QuestManagerComponent.Add Quest` _bp_questmanager "/Game/ARPG/Actor/Quest/BP_WorldQuest.BP_WorldQuest_C" false)))

(event `Key|Z`
  (params (Key :type "Key Structure")))

(event `Key|X`
  (params (Key :type "Key Structure")))

(event `Key|C`
  (params (Key :type "Key Structure"))
  (:`Pressed`
    (`self.AddXP` 150.0)))

(event `AddXP`
  (params (XP :type "Float (double-precision)"))
  (`/Game/ARPG/UI/WidgetBP/WB_Level.GainXP` (`/Game/ARPG/UI/WidgetBP/WB_MainPC.WB_Level` (`self.MainWidget`)) XP))

(event `Key|SpaceBar`
  (params (Key :type "Key Structure"))
  (:`Pressed`
    (if (not (`self.IsAttack`))
      (bind _counter (`/Engine/EditorBlueprintResources/StandardMacros.Do N` 2 :!label _label) ; 可以连跳2次
        (:`Exit`
          (switch `int` _counter
            (:`1`
              (`GameplayStatics.SpawnEmitterAtLocation` "/Game/Effects/FX_Particle/P_Sword_Trail_F.P_Sword_Trail_F" (`self.K2_GetActorLocation`))
              (`self.Jump`))
            (:`2`
              (`self.LaunchCharacter` (0.0 0.0 600.0))))
          (`GameplayStatics.PlaySoundAtLocation` "/Game/ARPG/Audio/Shinbi/Shinbi_Effort_Jump.Shinbi_Effort_Jump" (`self.K2_GetActorLocation`) (struct) 1.0 1.0 0.0 null null null))))))

(event `self.OnLanded`
  (params (Hit :type "HitResult Structure (by ref)"))
  (goto _label :!via `Reset`))

(event `Key|F`
  (params (Key :type "Key Structure"))
  (:`Pressed`
    (`self.OnInteracte`) ; 事件调度
    (for _array_element (`PrimitiveComponent.GetOverlappingActors` (`self.Box`) null)
      (if (`KismetSystemLibrary.DoesImplementInterface` _array_element "/Game/ARPG/Blueprints/Interface/BPI_Interaction.BPI_Interaction_C")
        (message `/Game/ARPG/Blueprints/Interface/BPI_Interaction.OnInteractWith` _array_element self) ; 蓝图接口
        (break)))))

(event `self.Box.OnComponentBeginOverlap`
  (params (OverlappedComponent :type "PrimitiveComponent Object Reference") (OtherActor :type "Actor Object Reference") (OtherComp :type "PrimitiveComponent Object Reference") (OtherBodyIndex :type Integer) (bFromSweep :type Boolean) (SweepResult :type "HitResult Structure (by ref)"))
  (if (`KismetSystemLibrary.DoesImplementInterface` OtherActor "/Game/ARPG/Blueprints/Interface/BPI_Interaction.BPI_Interaction_C")
    (set `self.Hit Other Actor` OtherActor)
    (message `/Game/ARPG/Blueprints/Interface/BPI_Interaction.BeginOverlapTargetObject` OtherActor)))

(event `self.Box.OnComponentEndOverlap`
  (params (OverlappedComponent :type "PrimitiveComponent Object Reference") (OtherActor :type "Actor Object Reference") (OtherComp :type "PrimitiveComponent Object Reference") (OtherBodyIndex :type Integer))
  (if (`KismetSystemLibrary.DoesImplementInterface` OtherActor "/Game/ARPG/Blueprints/Interface/BPI_Interaction.BPI_Interaction_C")
    (set `self.Hit Other Actor` null) ; 离开时置空
    (message `/Game/ARPG/Blueprints/Interface/BPI_Interaction.EndOverlapTargetObject` OtherActor)))

(event `Key|V`
  (params (Key :type "Key Structure"))
  (bind _subgoal_index (`self.Subgoal Index`))
  (bind _currentquest (`/Game/ARPG/Actor/Quest/QuestManagerComponent.CurrentQuest` (`self.BP_QuestManager`)))
  (:`Pressed`
    (`/Engine/EditorBlueprintResources/StandardMacros.IsValid` _currentquest
      (:`Is Valid`
        (`/Game/ARPG/Actor/Quest/BP_BaseQuest.Complete Sub Goal` _currentquest _subgoal_index true)
        (`/Engine/EditorBlueprintResources/StandardMacros.IncrementInt` _subgoal_index))
      (:`Is Not Valid`
        (`KismetSystemLibrary.PrintString` "当前任务为空")))))

(event `MeleeAttack`
  ;[1 1 1] 普通连击
  (if (`self.IsAttack`)
    (set `self.CanNextAttack` true) ; 第一次发起近战普攻后设为Ture，动画通知调用SaveAttac，就可以连击
    (else
      (set `self.IsAttack` true)
      (switch `int` (`self.AttackCount`) :!label _label_2
        (:`0`
          (set `self.AttackCount` 1)
          (`self.PlayAnimMontage` "/Game/ARPG/Charactors/Shinbi/Animation/Montage/Melee_B_Slow_Montage.Melee_B_Slow_Montage"))
        (:`1`
          (set `self.AttackCount` 2)
          (`self.PlayAnimMontage` "/Game/ARPG/Charactors/Shinbi/Animation/Montage/Melee_C_Slow_Montage.Melee_C_Slow_Montage"))
        (:`2`
          (set `self.AttackCount` 0) ; 重复循环普通攻击
          (`self.PlayAnimMontage` "/Game/ARPG/Charactors/Shinbi/Animation/Montage/Melee_D_Slow_Montage.Melee_D_Slow_Montage"))))))

(event `SaveAttack`
  ;[1 1 1] 普通连击
  (if (`self.CanNextAttack`)
    (set `self.CanNextAttack` false)
    (goto _label_2)))

(event `ResetCombo`
  ;[1 1 1] 普通连击
  (set `self.AttackCount` 0)
  (set `self.IsAttack` false)
  (set `self.CanNextAttack` false))

(event `Key|Q`
  (params (Key :type "Key Structure"))
  ;[1 1 1] 普通连击
  (:`Pressed`
    (if (`NavMovementComponent.IsFalling` (`self.CharacterMovement`))
      (`/Engine/EditorBlueprintResources/StandardMacros.DoOnce` false :!label _label_3
        (:`Completed`
          (bind _returnvalue (`self.PlayAnimMontage` "/Game/ARPG/Charactors/Shinbi/Animation/Montage/Melee_Air_Montage.Melee_Air_Montage")) ; 如果播放失败，则以秒为单位返回动画蒙太奇的长度
          (`KismetSystemLibrary.Delay` _returnvalue)
          (goto _label_3 :!via `Reset`)))
      (else
        (`self.MeleeAttack`)))))

(event `/Game/ARPG/Blueprints/Interface/BPI_Damage.ReceiveDamage`
  (params (CriticalChance :type "Float (single-precision)") (PhysicalDamage :type "Float (single-precision)") (CriticalDamage :type "Float (single-precision)") (MagicDamage :type "Float (single-precision)") (Attacker :type "Actor Object Reference"))
  ;[1 1 1] 收到伤害
  (bind (_critical _damage) (`self.CalculateDamage` PhysicalDamage MagicDamage CriticalChance CriticalDamage (`self.PhysicalDefence`) (`self.MagicDefence`) (`self.AbsoluteDefence`)))
  (`|ExecutionSequence`
    (:`then_0`
      (`self.PlayAnimMontage` "/Game/ARPG/Charactors/Shinbi/Animation/HitReact_Montage.HitReact_Montage" 1.0 (`KismetStringLibrary.Conv_StringToName` (`KismetStringLibrary.Conv_IntToString` (`KismetMathLibrary.RandomIntegerInRange` 0 3))))
      (`self.ResetCombo`))
    (:`then_1`
      (`self.ModifyAttribute` "NewEnumerator0" (* _damage -1.0) 0.0 _critical))))

(event `LineAttack`
  (bind _returnvalue (`self.K2_GetActorLocation`))
  (bind (_outhit _returnvalue_2) (`KismetSystemLibrary.LineTraceSingleForObjects` _returnvalue (+ _returnvalue (* (`self.GetActorForwardVector`) (`self.AttackRange`))) (`|MakeArray` "ObjectTypeQuery3" :!type "EObjectTypeQuery Enum"))) ; 沿给定的直线进行碰撞跟踪并返回遇到的第一个命中\n这只查找Objecttypes指定类型的对象
  (if _returnvalue_2
    (bind (_bblockinghit _binitialoverlap _time _distance _location _impactpoint _normal _impactnormal _physmat _hitactor) (`GameplayStatics.BreakHitResult` _outhit))
    (if (`KismetSystemLibrary.DoesImplementInterface` _hitactor "/Game/ARPG/Blueprints/Interface/BPI_Damage.BPI_Damage_C")
      (message `/Game/ARPG/Blueprints/Interface/BPI_Damage.ReceiveDamage` _hitactor (`self.CriticalDamage`) (`self.PhysicalDamage`) (`self.CriticalChance`) (`self.MagicDamage`) self))))

(event `Key|N`
  (params (Key :type "Key Structure")))

(fn `GetAttribute`
  (params (Key :type "/Game/ARPG/Blueprints/Enumeration/E_Attribute Enum" :default "NewEnumerator0"))
  (returns (Value :type "/Game/ARPG/Blueprints/Structure/S_Attribute Structure"))
  ;[0.9911 1 0] 纯函数
  (return (`BlueprintMapLibrary.Map_Find` (`self.Attributes`) Key)))

(fn `GetState`
  (returns (Attributes :type "Map of /Game/ARPG/Blueprints/Enumeration/E_Attribute Enum to /Game/ARPG/Blueprints/Structure/S_Attribute Structure") (Level :type Integer) (ReturnValue :type "Vector Structure"))
  (return (`self.Attributes`) (`self.Level`) (`self.K2_GetActorLocation`)))

(fn `HealthRegenTick`
  (bind ((`MaxValue_4_B105574A48990D433A33F4B15DC86C21` _maxvalue) (`RegenInterval_25_85F391B240D6E6B8ADDF62B5AA9742EC` _regeninterval) (`MaxRegenTime_27_B2B2638D48378D098D5378B3C5AAA47B` _maxregentime)) (break `/Game/ARPG/Blueprints/Structure/S_Attribute` (`self.GetAttribute` "NewEnumerator0")))
  (bind _returnvalue (* _maxvalue (/ _regeninterval _maxregentime)))
  (if (`self.IsFighting`)
    (`self.ModifyAttribute` "NewEnumerator0" (* _returnvalue 0.1))
    (else
      (`self.ModifyAttribute` "NewEnumerator0" _returnvalue))))

(fn `ManaRegenTick`
  (bind ((`MaxValue_4_B105574A48990D433A33F4B15DC86C21` _maxvalue) (`RegenInterval_25_85F391B240D6E6B8ADDF62B5AA9742EC` _regeninterval) (`MaxRegenTime_27_B2B2638D48378D098D5378B3C5AAA47B` _maxregentime)) (break `/Game/ARPG/Blueprints/Structure/S_Attribute` (`self.GetAttribute` "NewEnumerator1")))
  (bind _returnvalue (* _maxvalue (/ _regeninterval _maxregentime)))
  (if (`self.IsFighting`)
    (`self.ModifyAttribute` "NewEnumerator1" (* _returnvalue 0.1))
    (else
      (`self.ModifyAttribute` "NewEnumerator1" _returnvalue))))

(fn `ModifyAttribute`
  (params (Key :type "/Game/ARPG/Blueprints/Enumeration/E_Attribute Enum" :default "NewEnumerator3") (ModifyCurrenteV :type "Float (double-precision)") (MaxValue :type "Float (double-precision)") (IsCritical :type Boolean))
  (locals (LocalAttribute :type "/Game/ARPG/Blueprints/Enumeration/E_Attribute Enum" :default "NewEnumerator3") (LocalModifyValue :type Integer) (LocalMaxValue :type "Float (double-precision)"))
  (bind _localattribute (`local.LocalAttribute`))
  (bind _localmaxvalue (`local.LocalMaxValue`))
  (bind _returnvalue (`KismetMathLibrary.Conv_IntToDouble` (`local.LocalModifyValue`)))
  (bind ((`CurrenteValue_2_5120472D4ADFA7C850CAB88593C27016` _currentevalue) (`MaxValue_4_B105574A48990D433A33F4B15DC86C21` _maxvalue)) (break `/Game/ARPG/Blueprints/Structure/S_Attribute` (`self.GetAttribute` (`local.LocalAttribute`))))
  (set `local.LocalMaxValue` MaxValue)
  (bind _output_get (set `local.LocalAttribute` Key))
  (set `local.LocalModifyValue` (`KismetMathLibrary.FTrunc` (`KismetMathLibrary.FClamp` ModifyCurrenteV (* _currentevalue -1.0) (- _maxvalue _currentevalue))))
  (if (not (`|EnumEquality` _output_get "NewEnumerator2"))
    (bind _returnvalue_2 (`AddComponent|NODE_AddWC_OnDamage-0` :`bManualAttachment` true :`RelativeTransform` (`self.GetTransform`))) ; 手动附着
    (`/Game/ARPG/Component/WC_OnDamage.SetDamageText` _returnvalue_2 (`KismetMathLibrary.SelectFloat` _localmaxvalue _returnvalue (> _localmaxvalue 0.0)) (> _returnvalue 0.0) _localattribute IsCritical))
  (bind _value (`self.GetAttribute` _output_get))
  (bind (_currentevalue_2 _minvalue _maxvalue_2) (break `/Game/ARPG/Blueprints/Structure/S_Attribute` _value))
  (bind _returnvalue_3 (+ _maxvalue_2 _localmaxvalue))
  ;[1 1 1] 包成一个结构体
  (bind _structout (setmembers `/Game/ARPG/Blueprints/Structure/S_Attribute` :`StructRef` _value :`CurrenteValue` (`KismetMathLibrary.FClamp` (+ _currentevalue_2 _returnvalue) _minvalue _returnvalue_3) :`MaxValue` _returnvalue_3))
  ;[1 1 1] 和对应键值一起压进AttributeMap内存里去
  (`self.SetAttribute` _localattribute _structout)
  (`self.Updata Attribute` _localattribute)
  (`self.Regen on Off` _localattribute)
  (return))

(fn `Regen on Off`
  (params (Key :type "/Game/ARPG/Blueprints/Enumeration/E_Attribute Enum" :default "NewEnumerator3"))
  (bind ((`CurrenteValue_2_5120472D4ADFA7C850CAB88593C27016` _currentevalue) (`MaxValue_4_B105574A48990D433A33F4B15DC86C21` _maxvalue) (`RegenTimeHandle_33_B7285365470DF217D6331D9779404162` _regentimehandle)) (break `/Game/ARPG/Blueprints/Structure/S_Attribute` (`self.GetAttribute` Key)))
  (bind _returnvalue (`KismetSystemLibrary.K2_IsTimerPausedHandle` _regentimehandle))
  (if (and (!= _currentevalue _maxvalue) _returnvalue)
    (`KismetSystemLibrary.K2_UnPauseTimerHandle` _regentimehandle)
    (elif (and (== _currentevalue _maxvalue) (not _returnvalue))
      (`KismetSystemLibrary.K2_PauseTimerHandle` _regentimehandle))))

(fn `SetAttribute`
  (params (Key :type "/Game/ARPG/Blueprints/Enumeration/E_Attribute Enum" :default "NewEnumerator0") (Value :type "/Game/ARPG/Blueprints/Structure/S_Attribute Structure (by ref)"))
  (`BlueprintMapLibrary.Map_Add` (`self.Attributes`) Key Value)
  (return))

(fn `SetupAttributeBar`
  (bind _mainwidget (`self.MainWidget`))
  (bind _wb_charactorborder (`/Game/ARPG/UI/WidgetBP/WB_MainPC.WB_CharactorBorder` _mainwidget))
  (bind _structout (setmembers `/Game/ARPG/Blueprints/Structure/S_Attribute` :`StructRef` (`self.GetAttribute` "NewEnumerator0") :`GlassBallWidget` (`/Game/ARPG/UI/WidgetBP/WB_MainPC.Health` _mainwidget) :`HealthBar` (`/Game/ARPG/UI/WidgetBP/WB_CharactorBorder.WB_HealthBar` _wb_charactorborder)))
  (`self.SetAttribute` "NewEnumerator0" _structout)
  (bind _structout_2 (setmembers `/Game/ARPG/Blueprints/Structure/S_Attribute` :`StructRef` (`self.GetAttribute` "NewEnumerator1") :`GlassBallWidget` (`/Game/ARPG/UI/WidgetBP/WB_MainPC.Mana` _mainwidget) :`ManaBar` (`/Game/ARPG/UI/WidgetBP/WB_CharactorBorder.WB_ManaBar` _wb_charactorborder)))
  (`self.SetAttribute` "NewEnumerator1" _structout_2)
  (bind _structout_3 (setmembers `/Game/ARPG/Blueprints/Structure/S_Attribute` :`StructRef` (`self.GetAttribute` "NewEnumerator2") :`Stamina` (`/Game/ARPG/UI/WidgetBP/WB_CharactorBorder.Stamina` _wb_charactorborder)))
  (`self.SetAttribute` "NewEnumerator2" _structout_3))

(fn `StaminaRegen`
  (bind ((`MaxValue_4_B105574A48990D433A33F4B15DC86C21` _maxvalue) (`RegenInterval_25_85F391B240D6E6B8ADDF62B5AA9742EC` _regeninterval) (`MaxRegenTime_27_B2B2638D48378D098D5378B3C5AAA47B` _maxregentime)) (break `/Game/ARPG/Blueprints/Structure/S_Attribute` (`self.GetAttribute` "NewEnumerator2")))
  (bind _returnvalue (* _maxvalue (/ _regeninterval _maxregentime)))
  (if (`self.IsFighting`)
    (`self.ModifyAttribute` "NewEnumerator2" (* _returnvalue 0.1))
    (else
      (`self.ModifyAttribute` "NewEnumerator2" _returnvalue))))

(fn `Updata Attribute`
  (params (Key :type "/Game/ARPG/Blueprints/Enumeration/E_Attribute Enum" :default "NewEnumerator3"))
  (bind (_currentevalue _minvalue _maxvalue _glassballwidget _healthbar _manabar _stamina) (break `/Game/ARPG/Blueprints/Structure/S_Attribute` (`self.GetAttribute` Key)))
  (bind _glassball_img (`/Game/ARPG/UI/WidgetBP/WB_GlassBall.GlassBall_img` _glassballwidget))
  (bind _returnvalue (`KismetMathLibrary.FClamp` (/ _currentevalue _maxvalue)))
  (bind _result (`|FormatText` "{Current}/{Max}" (`KismetMathLibrary.Round` _currentevalue) (`KismetMathLibrary.Round` _maxvalue)))
  (switch `/Game/ARPG/Blueprints/Enumeration/E_Attribute` Key
    (:`NewEnumerator0`
      (`TextBlock.SetText` (`/Game/ARPG/UI/WidgetBP/WB_HealthBar.HealthText` _healthbar) _result)
      (`ProgressBar.SetPercent` (`/Game/ARPG/UI/WidgetBP/WB_HealthBar.HealthBar` _healthbar) _returnvalue)
      (bind _returnvalue_2 (`Image.GetDynamicMaterial` _glassball_img))
      (`MaterialInstanceDynamic.SetScalarParameterValue` _returnvalue_2 "Percent" _returnvalue) ; Scalar
      (`MaterialInstanceDynamic.SetVectorParameterValue` _returnvalue_2 "Color" (`KismetMathLibrary.LinearColorLerpUsingHSV` (struct :`R` 1.39 :`A` 1.0) (`/Game/ARPG/UI/WidgetBP/WB_GlassBall.Color` _glassballwidget) _returnvalue)))
    (:`NewEnumerator1`
      (`TextBlock.SetText` (`/Game/ARPG/UI/WidgetBP/WB_ManaBar.ManaText` _manabar) _result)
      (`ProgressBar.SetPercent` (`/Game/ARPG/UI/WidgetBP/WB_ManaBar.ManaBar` _manabar) _returnvalue)
      (bind _returnvalue_3 (`Image.GetDynamicMaterial` _glassball_img))
      (`MaterialInstanceDynamic.SetScalarParameterValue` _returnvalue_3 "Percent" _returnvalue) ; Scalar
    )
    (:`NewEnumerator2`
      (`ProgressBar.SetPercent` _stamina _returnvalue))))

(fn `UserConstructionScript`
  (`parent.UserConstructionScript`))