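; ARPG NPC that the player talks to for dialogue, quests and a food store.
; Special NPCs build a menu from DTConversation, with quest topics gated by player level; others show a random line in their interaction widget.
; Per-topic indices step through timed dialogue to choices that continue, go back, add or finish quests, or quit.
; On authority, it fills its inventory from DT_ItemList and serves it as a container to viewing players.
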(event `ContinueSelect`
  (params (SubgoalType :type "/Game/ARPG/Blueprints/Enumeration/E_SelectSubgoalType Enum" :default "NewEnumerator0"))
  (switch `/Game/ARPG/Blueprints/Enumeration/E_SelectSubgoalType` SubgoalType
    (:`NewEnumerator1`
      (`self.OnClickedContinue`))
    (:`NewEnumerator2`
      (`self.OnClickedBack`))
    (:`NewEnumerator5`
      (`self.OnBackToLastSelect`))
    (:`NewEnumerator3`
      (`self.OnClickedAddQuest`))
    (:`NewEnumerator6`
      (`self.OnFinishQuest`))
    (:`NewEnumerator4`
      (`self.OnClickedQuit`))))

(event `OnFinishQuest`
  (bind _shinbi (`self.Shinbi`))
  (bind ((`AmountToHunt_15_B17FCC6A4A55119EF8FC25809326EBB2` _amounttohunt) (`ItemInfo_49_186008B14DF0F1195E0873923D2B32FC` _iteminfo)) (break `/Game/ARPG/Actor/Quest/S_SubGoalInfo` (`/Game/ARPG/Actor/Quest/QuestManagerComponent.CurrentSubGoalInfo` (`self.BP_QuestManager`))))
  (`KismetArrayLibrary.Array_Remove` (`self.TalkSelectBorderInfo`) (`self.CurrentSelectTalkTypeIndex`)) ; 删除任务
  (`/Game/ARPG/Actor/Quest/WB_Quest.PlayQuest` (`/Game/ARPG/UI/WidgetBP/WB_MainPC.WB_Quest` (`/Game/ARPG/Charactors/Shinbi/BP_CharaShinbi.MainWidget` _shinbi)) false)
  (`self.OnClickedEndTalk`)
  (`/Game/ARPG/Actor/Item/C_InventoryManager.Client_Remove Item For Quest` (`/Game/ARPG/Blueprints/BP_PlayerControllerARPG.C_InventeryManager` (cast `/Game/ARPG/Blueprints/BP_PlayerControllerARPG` (`self.GetController` _shinbi) :!pure true)) _iteminfo _amounttohunt))

(event `OnClickedAddQuest`
  (`/Game/ARPG/Actor/Quest/QuestManagerComponent.Add Quest` (`/Game/ARPG/Charactors/BP_CharactorARPG.BP_QuestManager` (`self.Shinbi`)) (`.QuestInfo_8_BBC93E1940BC3EB2A99E56A4FD4936F6` (break `/Game/ARPG/Blueprints/Structure/S_Conversation` (`self.CurrentSelectTalkType`))) false)
  (`self.UpdateQuestInfo` true)
  (`self.OnClickedEndTalk`))

(event `OnBackToLastSelect`
  (bind (_talktypeinfo _talkinfo _questinfo _talktype _suggestlevel _hasreceivequest _receivetalktypeinfo _receivequesttalkinfo) (break `/Game/ARPG/Blueprints/Structure/S_Conversation` (`self.CurrentSelectTalkType`)))
  (bind _output (`|GetArrayItem` (`self.DTTalkInfoIndex`) (`self.CurrentSelectTalkTypeIndex`)))
  (bind _mainwidget (`/Game/ARPG/Charactors/Shinbi/BP_CharaShinbi.MainWidget` (`self.Shinbi`)))
  (`PanelWidget.ClearChildren` (`/Game/ARPG/UI/WidgetBP/WB_MainPC.SelectTalkInfoScrollBox` _mainwidget))
  (`/Game/ARPG/UI/WidgetBP/WB_TalkBorder.Hide` (`/Game/ARPG/UI/WidgetBP/WB_MainPC.WB_TalkBorder` _mainwidget))
  (for (_array_element _array_index) (`.SelectSubgoalInfo_14_B609088C4E0C5BB780EA39AD9D5642DC` (break `/Game/ARPG/Blueprints/Structure/S_SpeechContent` (select `bool` _hasreceivequest :`false` (`|GetArrayItem` _talkinfo _output) :`true` (`|GetArrayItem` _receivequesttalkinfo _output)))) :!label _label
    (bind (_talksubgoalinfo _seletsubgoaltype) (break `/Game/ARPG/Blueprints/Structure/S_SelectSubgoalInfo` _array_element))
    (bind _returnvalue (`|CreateWidget` "/Game/ARPG/UI/WidgetBP/WB_TalkInfo.WB_TalkInfo_C" null self _talksubgoalinfo _array_index "NewEnumerator0" _seletsubgoaltype))
    (`PanelWidget.AddChild` (`/Game/ARPG/UI/WidgetBP/WB_MainPC.SelectTalkInfoScrollBox` (`/Game/ARPG/Charactors/Shinbi/BP_CharaShinbi.MainWidget` (`self.Shinbi`))) _returnvalue)))

(event `SkipTalkInfo`
  (bind _dttalkinfoindex (`self.DTTalkInfoIndex`))
  (bind (_talktypeinfo _talkinfo _questinfo _talktype _suggestlevel _hasreceivequest _receivetalktypeinfo _receivequesttalkinfo) (break `/Game/ARPG/Blueprints/Structure/S_Conversation` (`self.CurrentSelectTalkType`)))
  (bind _output (`|GetArrayItem` _dttalkinfoindex (`self.CurrentSelectTalkTypeIndex`)))
  (bind _output_2 (`|GetArrayItem` _talkinfo _output))
  (bind _returnvalue (select `bool` _hasreceivequest :`false` _output_2 :`true` (`|GetArrayItem` _receivequesttalkinfo _output)))
  (bind (_hassubgoalselect _talkername _talkerintro _speechinfo _showinfoduration _selectsubgoalinfo) (break `/Game/ARPG/Blueprints/Structure/S_SpeechContent` _returnvalue))
  (if (not _hassubgoalselect)
    (if _hassubgoalselect :!label _label_2
      (goto _label)
      (else
        (`KismetArrayLibrary.Array_Set` _dttalkinfoindex (`self.CurrentSelectTalkTypeIndex`) (+ (select `bool` _hasreceivequest :`false` (`KismetArrayLibrary.Array_Find` _talkinfo _output_2) :`true` (`KismetArrayLibrary.Array_Find` _receivequesttalkinfo _returnvalue)) 1))
        (`/Game/ARPG/UI/WidgetBP/WB_TalkBorder.PopUp ` (`/Game/ARPG/UI/WidgetBP/WB_MainPC.WB_TalkBorder` (`/Game/ARPG/Charactors/Shinbi/BP_CharaShinbi.MainWidget` (`self.Shinbi`))) _talkername _speechinfo _talkerintro self :!label _label_3)
        (`KismetSystemLibrary.Delay` _showinfoduration)
        (goto _label_2)))))

(event `OnClickedContinue`
  (bind (_talktypeinfo _talkinfo _questinfo _talktype _suggestlevel _hasreceivequest _receivetalktypeinfo _receivequesttalkinfo) (break `/Game/ARPG/Blueprints/Structure/S_Conversation` (`self.CurrentSelectTalkType`)))
  (bind _output (`|GetArrayItem` (`self.DTTalkInfoIndex`) (`self.CurrentSelectTalkTypeIndex`)))
  (bind _output_2 (`|GetArrayItem` _talkinfo _output))
  (`KismetArrayLibrary.Array_Set` (`self.DTTalkInfoIndex`) (`self.CurrentSelectTalkTypeIndex`) (+ (select `bool` _hasreceivequest :`false` (`KismetArrayLibrary.Array_Find` _talkinfo _output_2) :`true` (`KismetArrayLibrary.Array_Find` _receivequesttalkinfo (select `bool` _hasreceivequest :`false` _output_2 :`true` (`|GetArrayItem` _receivequesttalkinfo _output)))) 1))
  (`PanelWidget.ClearChildren` (`/Game/ARPG/UI/WidgetBP/WB_MainPC.SelectTalkInfoScrollBox` (`/Game/ARPG/Charactors/Shinbi/BP_CharaShinbi.MainWidget` (`self.Shinbi`))) :!label _label_4)
  (goto _label_3))

(event `OnClickedQuestInfo`
  (goto _label_4))

(event `OnClickedGoodsStore`)

(event `OnClickedEndTalk`
  (bind _mainwidget (`/Game/ARPG/Charactors/Shinbi/BP_CharaShinbi.MainWidget` (`self.Shinbi`)))
  (`PanelWidget.ClearChildren` (`/Game/ARPG/UI/WidgetBP/WB_MainPC.SelectTalkInfoScrollBox` _mainwidget) :!label _label_5)
  (`/Game/ARPG/UI/WidgetBP/WB_TalkBorder.Hide` (`/Game/ARPG/UI/WidgetBP/WB_MainPC.WB_TalkBorder` _mainwidget)))

(event `OnClickedWeaponStore`)

(event `OnClickedQuit`
  (goto _label_5))

(event `OnClickedElseInfo`)

(event `OnClickedTalkTypeInfo`
  (params (TalkTypeIndex :type Integer))
  (set `self.CurrentSelectTalkTypeIndex` TalkTypeIndex)
  (bind _output_get (set `self.CurrentSelectTalkType` (`|GetArrayItem` (`self.TalkSelectBorderInfo`) TalkTypeIndex)))
  (switch `/Game/ARPG/Blueprints/Enumeration/E_TalkType` (`.TalkType_11_C199EE084AED66B7DF648F87F2E66A5A` (break `/Game/ARPG/Blueprints/Structure/S_Conversation` _output_get))
    (:`NewEnumerator0`
      (`self.OnClickedElseInfo`))
    (:`NewEnumerator1`
      (`self.OnClickedQuestInfo`))
    (:`NewEnumerator5`
      (`self.OnClickedFoodStore`))
    (:`NewEnumerator6`
      (`self.OnClickedEndTalk`))))

(event `OnClickedFoodStore`
  (message `/Game/ARPG/Actor/Item/BPI_HUD.UIOpen Food Store` (`GameplayStatics.GetPlayerController` 0) self)
  (`self.OnClickedEndTalk`) ; 打开商店后要关闭对话
)

(event `OnClickedBack`
  (bind _mainwidget (`/Game/ARPG/Charactors/Shinbi/BP_CharaShinbi.MainWidget` (`self.Shinbi`)))
  (`PanelWidget.ClearChildren` (`/Game/ARPG/UI/WidgetBP/WB_MainPC.SelectTalkInfoScrollBox` _mainwidget))
  (`/Game/ARPG/UI/WidgetBP/WB_TalkBorder.Hide` (`/Game/ARPG/UI/WidgetBP/WB_MainPC.WB_TalkBorder` _mainwidget))
  (`KismetArrayLibrary.Array_Clear` (`self.WBTalkInfo`) :!label _label_6)
  (`KismetArrayLibrary.Array_Clear` (`self.DTTalkInfoIndex`))
  (for (_array_element _array_index) (`self.TalkSelectBorderInfo`)
    (bind (_talktypeinfo _talkinfo _questinfo _talktype _suggestlevel _hasreceivequest _receivetalktypeinfo) (break `/Game/ARPG/Blueprints/Structure/S_Conversation` _array_element))
    (if (`|EnumEquality` _talktype "NewEnumerator1")
      (if (and (>= (`self.ShinbiLevel`) _suggestlevel) (`KismetSystemLibrary.IsValidClass` _questinfo))
        (bind _returnvalue (`|CreateWidget` "/Game/ARPG/UI/WidgetBP/WB_TalkInfo.WB_TalkInfo_C" null self (select `bool` _hasreceivequest :`false` _talktypeinfo :`true` _receivetalktypeinfo) _array_index _talktype :!label _label_7))
        (`KismetArrayLibrary.Array_Add` (`self.WBTalkInfo`) _returnvalue)
        (`PanelWidget.AddChild` (`/Game/ARPG/UI/WidgetBP/WB_MainPC.SelectTalkInfoScrollBox` (`/Game/ARPG/Charactors/Shinbi/BP_CharaShinbi.MainWidget` (`self.Shinbi`))) _returnvalue)
        (`KismetArrayLibrary.Array_Add` (`self.DTTalkInfoIndex`)))
      (else
        (goto _label_7)))))

(event `/Game/ARPG/Blueprints/Interface/BPI_Interaction.OnInteractWith`
  (params (Character :type "/Game/ARPG/Charactors/Shinbi/BP_CharaShinbi Object Reference"))
  (bind _randominfo (`self.RandomInfo`))
  (bind _aswb_interaction (cast `/Game/ARPG/UI/WidgetBP/WB_Interaction` (`WidgetComponent.GetWidget` (`self.WC_Interact`)) :!pure true))
  (if (`self.IsSpecial`)
    (if (not (`PanelWidget.HasAnyChildren` (`/Game/ARPG/UI/WidgetBP/WB_MainPC.SelectTalkInfoScrollBox` (`/Game/ARPG/Charactors/Shinbi/BP_CharaShinbi.MainWidget` (`self.Shinbi`)))))
      (goto _label_6))
    (elif (not (`/Game/ARPG/UI/WidgetBP/WB_Interaction.IsTalking` _aswb_interaction))
      (`/Game/ARPG/UI/WidgetBP/WB_Interaction.ShowTalkInfo` _aswb_interaction (`|GetArrayItem` _randominfo (`KismetMathLibrary.RandomInteger` (`KismetArrayLibrary.Array_Length` _randominfo)))))))

(event `/Game/ARPG/Blueprints/Interface/BPI_Interaction.BeginOverlapTargetObject`
  (`SceneComponent.SetVisibility` (`self.WC_Interact`) true false))

(event `/Game/ARPG/Blueprints/Interface/BPI_Interaction.EndOverlapTargetObject`
  (`SceneComponent.SetVisibility` (`self.WC_Interact`) false false))

(event `self.Sphere.OnComponentBeginOverlap`
  (params (OverlappedComponent :type "PrimitiveComponent Object Reference") (OtherActor :type "Actor Object Reference") (OtherComp :type "PrimitiveComponent Object Reference") (OtherBodyIndex :type Integer) (bFromSweep :type Boolean) (SweepResult :type "HitResult Structure (by ref)"))
  (if (== OtherActor (`self.Shinbi`))
    (`SceneComponent.SetHiddenInGame` (`self.WC_Interact`) false false)))

(event `self.Sphere.OnComponentEndOverlap`
  (params (OverlappedComponent :type "PrimitiveComponent Object Reference") (OtherActor :type "Actor Object Reference") (OtherComp :type "PrimitiveComponent Object Reference") (OtherBodyIndex :type Integer))
  (if (== OtherActor (`self.Shinbi`))
    (`SceneComponent.SetHiddenInGame` (`self.WC_Interact`) true false)))

(event `self.ReceiveBeginPlay`
  (bind _dt_conversation (`self.DT_Conversation`))
  (bind _shinbi (`self.Shinbi`))
  (`parent.ReceiveBeginPlay`)
  (bind _asbp_chara_shinbi (cast `/Game/ARPG/Charactors/Shinbi/BP_CharaShinbi` (`GameplayStatics.GetPlayerCharacter` 0)))
  (set `self.Shinbi` _asbp_chara_shinbi)
  (`self.SetOwner` _asbp_chara_shinbi)
  (`PrimitiveComponent.SetOwnerNoSee` (`self.PaperSprite`) true)
  (bind _aswb_interaction (cast `/Game/ARPG/UI/WidgetBP/WB_Interaction` (`WidgetComponent.GetUserWidgetObject` (`self.WC_Interact`))))
  (`TextBlock.SetText` (`/Game/ARPG/UI/WidgetBP/WB_Interaction.Name` _aswb_interaction) (`self.Name`))
  (`SceneComponent.SetVisibility` (`self.PaperSprite`) true false)
  (add `/Game/ARPG/Charactors/Shinbi/BP_CharaShinbi.UpgradeForQuest` _shinbi (`|CreateDelegate` :!event `UpdateQuest`))
  (`self.UpdateQuest` (`/Game/ARPG/Charactors/Shinbi/BP_CharaShinbi.Level` _shinbi))
  (`/Engine/EditorBlueprintResources/StandardMacros.IsValid` _dt_conversation
    (:`Is Valid`
      (bind _outrownames (`DataTableFunctionLibrary.GetDataTableRowNames` _dt_conversation)) ; 获取数据表行名称
      (for _array_element _outrownames
        (bind _returnvalue (`|GetDataTableRow` (`self.DT_Conversation`) _array_element) ; 尝试通过数据表的行名从数据表中检索TableRow
          (:`then`
            (`KismetArrayLibrary.Array_Add` (`self.TalkSelectBorderInfo`) _returnvalue))))
      (`self.InitializeInventory`))))

(event `UpdateQuest`
  (params (Level :type Integer))
  (set `self.ShinbiLevel` Level))

(fn `Get Container Properties`
  (returns (Name :type Text) (InventorySize :type Integer) (InventoryType :type "/Game/ARPG/Actor/Item/E_InventoryTy Enum"))
  (return (`self.StoreName`) (`self.Inventory Size`) "NewEnumerator1") ; 而玩家的默认就是PlayerInventory，就不用去改了
)

(fn `Get Food Store List`
  (returns (LocalInventoryItem :type "Array of /Game/ARPG/Actor/Item/S_InventoryItem Structure"))
  (locals (LInventoryItem :type "Array of /Game/ARPG/Actor/Item/S_InventoryItem Structure"))
  (bind _outrownames (`DataTableFunctionLibrary.GetDataTableRowNames` "/Game/ARPG/Actor/Item/DT_ItemList.DT_ItemList"))
  (for _array_element _outrownames
    (bind _returnvalue (`|GetDataTableRow` "/Game/ARPG/Actor/Item/DT_ItemList.DT_ItemList" _array_element)
      (:`then`
        (bind ((`ItemType_18_8EDF4F664BC6073C3C63508C99CF45DF` _itemtype) (`MaxStackSize_30_007273284253E7C24F0E0F8B1D09C34C` _maxstacksize)) (break `/Game/ARPG/Actor/Item/S_InventoryItem` _returnvalue))
        (if (`|EnumEquality` _itemtype "NewEnumerator5")
          (bind _structout (setmembers `/Game/ARPG/Actor/Item/S_InventoryItem` :`StructRef` _returnvalue :`Amount` _maxstacksize))
          (`KismetArrayLibrary.Array_Add` (`local.LInventoryItem`) _structout)))))
  (return (`local.LInventoryItem`)) ; 返回商品列表
)

(fn `GetContainerInventory`
  (returns (InventoryConponent :type "/Game/ARPG/Actor/Item/C_Inventory Object Reference"))
  (return (`self.C_Inventery`)))

(fn `GetPlayerViewing`
  (returns (PlayerViewing :type "Array of PlayerState Object Reference"))
  (return (`self.Player Viewing`)) ; 存储所有客户端连接过来的状态
)

(fn `InitializeInventory`
  (returns (Success :type Boolean))
  (`/Engine/EditorBlueprintResources/ActorMacros.Switch Has Authority`
    (:`Authority`
      (bind _localinventoryitem (`self.Get Food Store List`)) ; 获得商品列表
      (`self.Load Inventory Items` (`self.Inventory Size`) _localinventoryitem) ; 加载商品，加载到Inventory组件
      (return true))
    (:`Remote`
      (return false))))

(fn `Load Inventory Items`
  (params (InventorySize :type Integer) (InventoryItems :type "Array of /Game/ARPG/Actor/Item/S_InventoryItem Structure"))
  (returns (Success :type Boolean))
  (`/Engine/EditorBlueprintResources/ActorMacros.Switch Has Authority`
    (:`Authority`
      (bind _output_get (set `self.Inventory Size` InventorySize))
      (`/Game/ARPG/Actor/Item/C_Inventory.Load Inventory Item` (`self.C_Inventery`) _output_get InventoryItems)
      (return true))
    (:`Remote`
      (return false))))

(fn `On Actor Used`
  (params (Controller :type "PlayerController Object Reference"))
  (returns (Success :type Boolean))
  (`/Engine/EditorBlueprintResources/ActorMacros.Switch Has Authority`
    (:`Authority`
      (bind _asbp_player_controller_arpg (cast `/Game/ARPG/Blueprints/BP_PlayerControllerARPG` Controller)
        (:`then`
          (`KismetArrayLibrary.Array_Add` (`self.Player Viewing`) (`Controller.PlayerState` _asbp_player_controller_arpg))
          (`/Game/ARPG/Actor/Item/C_InventoryManager.Server_UseContainer` (`/Game/ARPG/Blueprints/BP_PlayerControllerARPG.C_InventeryManager` _asbp_player_controller_arpg) self)
          (return true))
        (:`CastFailed`
          _)))
    (:`Remote`
      _))
  (return false))

(fn `UpdateQuestInfo`
  (params (HasReceiveQuest :type Boolean))
  (bind _currentselecttalktypeindex (`self.CurrentSelectTalkTypeIndex`))
  (bind _talkselectborderinfo (`self.TalkSelectBorderInfo`))
  (bind _structout (setmembers `/Game/ARPG/Blueprints/Structure/S_Conversation` :`StructRef` (`|GetArrayItem` _talkselectborderinfo _currentselecttalktypeindex) :`HasReceiveQuest` HasReceiveQuest))
  (`KismetArrayLibrary.Array_Set` _talkselectborderinfo _currentselecttalktypeindex _structout))

(fn `UserConstructionScript`
  (`parent.UserConstructionScript`)
  (`/Engine/EditorBlueprintResources/ActorMacros.Switch Has Authority`
    (:`Authority`
      (`/Game/ARPG/Actor/Item/C_Inventory.Server_InitialInventory` (`self.C_Inventery`) (`self.Inventory Size`)) ; 设置商店有多少个Slot
    )))